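; Blueprint component for mounted VR weapons that drives a dummy gripping hand and locks the player's IK hand to it.
; It binds to the gun's trigger pulled and released events to switch the dummy hand's RightHand_AnimBP between resting and trigger-pull grip poses.
; It also sets or clears the dummy hand on the motion controller as the IK target, stopping the hand rotating freely while the gun is grabbed.
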(event `Dummy hand trigger pull animation`
  (params (BP_Gun :type "/Game/VR_Weapons/Global/Blueprints/BP_Gun Object Reference") (`Dummy hand` :type "SkeletalMeshComponent Object Reference") (Weapon :type "/Game/VR_Weapons/Pawn/Blueprints/E_WeaponType Enum" :default "NewEnumerator0"))
  (set `self.Weapon` Weapon)
  (add `/Game/VR_Weapons/Global/Blueprints/BP_Gun.Weapon trigger pulled` BP_Gun (delegate `Weapon trigger pulled_Event`))
  (add `/Game/VR_Weapons/Global/Blueprints/BP_Gun.Weapon trigger released` BP_Gun (delegate `Weapon trigger released_Event`))
  ;[0 0 0] update animation of dummy grip hand
  (bind _asright_hand_anim_bp (cast `/Game/VR_Weapons/Pawn/Mannequin/Animations/RightHand_AnimBP` (`SkeletalMeshComponent.GetAnimInstance` `Dummy hand`) :!label _label))
  (set `/Game/VR_Weapons/Pawn/Mannequin/Animations/RightHand_AnimBP.GripState` "NewEnumerator2" _asright_hand_anim_bp) ; resting position
  (set `/Game/VR_Weapons/Pawn/Mannequin/Animations/RightHand_AnimBP.WeaponState` (`self.Weapon`) _asright_hand_anim_bp)
  (set `/Game/VR_Weapons/Pawn/Mannequin/Animations/RightHand_AnimBP.PrimaryGrip` true _asright_hand_anim_bp))

(event `Weapon trigger released_Event`
  ;[0 0 0] update animation of dummy grip hand
  (goto _label))

(event `Weapon trigger pulled_Event`
  ;[0 0 0] update animation of dummy grip hand
  (bind _asright_hand_anim_bp (cast `/Game/VR_Weapons/Pawn/Mannequin/Animations/RightHand_AnimBP` (`SkeletalMeshComponent.GetAnimInstance` (stale `Dummy hand trigger pull animation` `Dummy hand`))))
  (set `/Game/VR_Weapons/Pawn/Mannequin/Animations/RightHand_AnimBP.GripState` "NewEnumerator4" _asright_hand_anim_bp) ; trigger pull
  (set `/Game/VR_Weapons/Pawn/Mannequin/Animations/RightHand_AnimBP.WeaponState` (`self.Weapon`) _asright_hand_anim_bp)
  (set `/Game/VR_Weapons/Pawn/Mannequin/Animations/RightHand_AnimBP.PrimaryGrip` true _asright_hand_anim_bp))

(fn `Set IK Target as Dummy Hand`
  (params (`Primary motion controller BP` :type "/Game/VR_Weapons/Pawn/Blueprints/BP_MotionController Object Reference") (DummyGrippingHand :type "SkeletalMeshComponent Object Reference") (`Remove IK target` :type Boolean))
  (bind _primary_motion_controller_bp (`local.Primary motion controller BP`))
  (`/Engine/EditorBlueprintResources/StandardMacros.IsValid` `Primary motion controller BP`
    (:`Is Valid`
      (if `Remove IK target`
        ;[0.6302 0.2091 0] remove IK target when gun is released
        (set `/Game/VR_Weapons/Pawn/Blueprints/BP_MotionController.DummyGrippingHand` null _primary_motion_controller_bp)
        (set `/Game/VR_Weapons/Pawn/Blueprints/BP_MotionController.MountedGunGrabbed` false _primary_motion_controller_bp)
        (else
          ;[0.6302 0.2091 0] Set IK target as Dummy hand to stop IK/motion controller hand rotating freely while gun is mounted
          (set `/Game/VR_Weapons/Pawn/Blueprints/BP_MotionController.DummyGrippingHand` DummyGrippingHand _primary_motion_controller_bp) ; Dummy hand is set in BP_MotionController\nThen the IK system gets updated in MotionControllerPawn's "update hand position" graph\nwhere the IK hand is overriden using the orientation of the Dummy hand to "lock" it in place and stop it rotating freely
          (set `/Game/VR_Weapons/Pawn/Blueprints/BP_MotionController.MountedGunGrabbed` true _primary_motion_controller_bp))))
    (:`Is Not Valid`)))