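; Laser sight component for VR weapons that draws a beam and an end-point dot where the weapon's laser lands.
; InitialiseLaser stores the beam mesh and dot passed in by the caller.
; UpdateLaser, not ticked by the component itself, line-traces forward on Visibility, then stretches the beam's X scale to the hit distance and moves the dot there.
; Without a hit, both extend to the maximum trace range.
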(fn `Initialise laser`
  (params (LaserBeamMesh :type "SceneComponent Object Reference") (LaserEndPointDot :type "SceneComponent Object Reference"))
  (set `self.Laser Mesh` LaserBeamMesh)
  (set `self.Laser End Point Dot` LaserEndPointDot))

(fn `Update laser`
  (bind _laser_end_point_dot (`self.Laser End Point Dot`))
  (bind _returnvalue (`SceneComponent.K2_GetComponentLocation` (`self.Laser Mesh`)))
  (bind (_returnvalue_x _returnvalue_y _returnvalue_z) (`KismetMathLibrary.BreakVector` (`SceneComponent.K2_GetComponentScale` (`self.Laser mesh`))))
  (bind _returnvalue_2 (+ _returnvalue (* (`KismetMathLibrary.GetForwardVector` (`SceneComponent.K2_GetComponentRotation` (`self.Laser Mesh`))) 10000.0)))
  (bind (_outhit _returnvalue_3) (`KismetSystemLibrary.LineTraceSingle` :`Start` _returnvalue :`End` _returnvalue_2 :`TraceChannel` "TraceTypeQuery1" :`bTraceComplex` true :`DrawTime` 0.0))
  (`SceneComponent.SetVisibility` (`self.Laser mesh`) true true)
  (`SceneComponent.SetVisibility` (`self.Laser End Point Dot`) true true)
  (if _returnvalue_3
    (bind (_bblockinghit _binitialoverlap _time _distance _location) (`GameplayStatics.BreakHitResult` _outhit))
    (`SceneComponent.SetWorldScale3D` (`self.Laser mesh`) (`KismetMathLibrary.MakeVector` (* _distance 0.01) _returnvalue_y _returnvalue_z))
    (`SceneComponent.K2_SetWorldLocation` _laser_end_point_dot _location false false)
    (else
      (`SceneComponent.SetWorldScale3D` (`self.Laser mesh`) (`KismetMathLibrary.MakeVector` 100.0 _returnvalue_y _returnvalue_z))
      (`SceneComponent.K2_SetWorldLocation` _laser_end_point_dot _returnvalue_2 false false))))