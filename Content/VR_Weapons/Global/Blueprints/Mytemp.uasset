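; Test actor in the VR weapons folder that snaps a referenced Bipod actor onto the surface beneath it.
; The construction script traces 100 units down, moves the Bipod to the impact point and debug-draws and prints the normal.
; It derives roll and pitch from the normal with atan2, then re-applies the saved yaw as a local rotation.
; The event graph is empty, and alternative transform experiments are left disconnected.
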(event `hit target`
  (params (`hit points` :type Integer)))

(fn `UserConstructionScript`
  (locals (yaw :type "Float (double-precision)" :default 0.0))
  (bind _returnvalue (`self.K2_GetActorLocation`))
  (bind _bipod (`self.Bipod`))
  (bind _bipod_2 (`self.Bipod`))
  (bind (_returnvalue_roll _returnvalue_pitch _returnvalue_yaw) (`KismetMathLibrary.BreakRotator` (`self.K2_GetActorRotation` _bipod_2)))
  (bind _outhit (`KismetSystemLibrary.LineTraceSingle` :`Start` _returnvalue :`End` (- _returnvalue (0.0 0.0 100.0)) :`TraceChannel` "TraceTypeQuery1" :`DrawDebugType` "ForDuration" :`DrawTime` 0.2))
  (bind (_bblockinghit _binitialoverlap _time _distance _location _impactpoint _normal) (`GameplayStatics.BreakHitResult` _outhit))
  (`KismetSystemLibrary.DrawDebugLine` _impactpoint (+ _impactpoint (* _normal 25.0)) (struct :`R` 1.0 :`G` 0.233938 :`A` 1.0) 0.2 1.0)
  (`KismetSystemLibrary.PrintString` (`KismetStringLibrary.Conv_DoubleToString` (.z _normal)) true true (struct :`R` 1.0 :`G` 0.138958 :`A` 1.0) 1.0)
  (`self.K2_SetActorLocation` _bipod_2 _impactpoint false false)
  (set `local.yaw` _returnvalue_yaw)
  (bind _z (.z _normal))
  (`self.K2_SetActorRelativeRotation` _bipod (`KismetMathLibrary.MakeRotator` (`KismetMathLibrary.DegAtan2` (.y _normal) _z) (* (`KismetMathLibrary.DegAtan2` (.x _normal) _z) -1.0)) false false)
  (`self.K2_AddActorLocalRotation` _bipod (`KismetMathLibrary.MakeRotator` 0.0 0.0 (`local.yaw`)) false false))