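; BP_MachineGunExample is a BP_Gun child for a mountable VR machine gun, in the turret example.
; Pickup while mounted sets the right dummy hand as the IK target through BPCMountedGunDummyHand, locking the hand to the gun.
; Dropping or releasing while mounted clears that target, and dropping also hides the dummy hand.
; ReadyToFire always returns true, and PlayHaptics loops a fixed automatic-fire rumble on the primary controller.
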(event `self.ReceiveBeginPlay`
  (`parent.ReceiveBeginPlay`)
  ;[0 0 0] Called in parent: BP_Gun
  (add `self.Weapon dropped` (delegate `Weapon dropped_Event`))
  (add `self.Weapon released while mounted` (delegate `Released while mounted`))
  (add `self.Weapon picked up` (delegate `Weapon picked up_Event`))
  (`/Game/VR_Weapons/Global/Blueprints/BPC_MountedGunDummyHand.Dummy hand trigger pull animation` (`self.BPC_MountedGunDummyHand`) self (`self.Dummy Hand Right`) "NewEnumerator3"))

(event `Released while mounted`
  ;[0 0 0] Called in parent: BP_Gun
  (`/Game/VR_Weapons/Global/Blueprints/BPC_MountedGunDummyHand.Set IK Target as Dummy Hand` (`self.BPC_MountedGunDummyHand`) (`self.Primary Motion Controller BP`) (`self.Dummy Hand Right`) true :!label _label))

(event `Weapon dropped_Event`
  (`SceneComponent.SetVisibility` (`self.Dummy Hand Right`) false false)
  (goto _label))

(event `Weapon picked up_Event`
  (if (`self.Weapon mounted`)
    (`/Game/VR_Weapons/Global/Blueprints/BPC_MountedGunDummyHand.Set IK Target as Dummy Hand` (`self.BPC_MountedGunDummyHand`) (`self.Primary Motion Controller BP`) (`self.Dummy Hand Right`) false)))

(fn `Play Haptics `
  (params (`Primary controller Intensity` :type "Float (double-precision)") (`Secondary controller intensity` :type "Float (double-precision)") (HapticEffect :type "HapticFeedbackEffect_Base Object Reference") (bLoop :type Boolean))
  (`/Game/VR_Weapons/Pawn/Blueprints/BP_MotionController.RumbleController` (`self.Primary Motion Controller BP`) "/Game/VR_Weapons/Pawn/Haptics/Haptics_auto.Haptics_auto" 1.0 true))

(fn `Ready to fire`
  (returns (`Weapon ready` :type Boolean))
  (return true))

(fn `Set IK target as pistol grip dummy hand`
  (params (Condition :type Boolean))
  (bind _debug_mode (`self.Debug mode`))
  (bind _primary_motion_controller_bp (`self.Primary Motion Controller BP`))
  (`/Engine/EditorBlueprintResources/StandardMacros.IsValid` _primary_motion_controller_bp
    (:`Is Valid`
      (if Condition
        ;[0.6302 0.2091 0] remove IK target when gun is released
        (set `/Game/VR_Weapons/Pawn/Blueprints/BP_MotionController.DummyGrippingHand` null _primary_motion_controller_bp)
        (set `/Game/VR_Weapons/Pawn/Blueprints/BP_MotionController.MountedGunGrabbed` false _primary_motion_controller_bp)
        (else
          ;[0.6302 0.2091 0] Set IK target as Dummy hand to stop IK/motion controller hand rotating freely while gun is mounted
          (set `/Game/VR_Weapons/Pawn/Blueprints/BP_MotionController.DummyGrippingHand` (`self.Dummy Hand Right`) _primary_motion_controller_bp) ; Dummy hand is set in BP_MotionController\nThen the IK system gets updated in MotionControllerPawn's "update hand position" graph\nwhere the IK hand is overriden using the orientation of the Dummy hand to "lock" it in place and stop it rotating freely
          (set `/Game/VR_Weapons/Pawn/Blueprints/BP_MotionController.MountedGunGrabbed` true _primary_motion_controller_bp))))
    (:`Is Not Valid`
      (`KismetSystemLibrary.PrintString` "BP Sniper: Primary motion controller BP not set!" _debug_mode _debug_mode (struct :`R` 1.0 :`A` 1.0) 5.0))))

(fn `Toggle mounted gun dummy hand visibility`
  (params (`New visibility` :type Boolean))
  (`SceneComponent.SetVisibility` (`self.Dummy Hand Right`) `New visibility` false) ; Hide/show fake motion controller mesh
)

(fn `UserConstructionScript`
  (`parent.UserConstructionScript`))