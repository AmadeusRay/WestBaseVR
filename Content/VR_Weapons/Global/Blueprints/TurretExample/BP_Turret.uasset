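; BP_Turret is an example VR turret that acts as a permanent bipod-style mount for a machine gun.
; On BeginPlay, after a short delay, it snaps the overlapping BP_MachineGunExample to a dummy, registers as its bipod and binds its fire and release events.
; Mounted-transform updates split pitch and yaw across two nested pivots, with an optional clamped slider rail.
; RangeBeforeDetaching always returns false, so the gun never detaches.
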(event `self.ReceiveBeginPlay`
  (bind _output (`|GetArrayItem` (`PrimitiveComponent.GetOverlappingActors` (`self.attach collision`) "/Game/VR_Weapons/Global/Blueprints/TurretExample/BP_MachineGunExample.BP_MachineGunExample_C")))
  (`parent.ReceiveBeginPlay`)
  (`KismetSystemLibrary.Delay` 0.5)
  (`self.K2_AttachToComponent` _output (`self.Attach dummy`) "None" "SnapToTarget" "SnapToTarget" "KeepRelative" true)
  (set `self.Mounted` true)
  (bind _asbp_gun (cast `/Game/VR_Weapons/Global/Blueprints/BP_Gun` _output))
  (bind _output_get (set `self.BP gun` _asbp_gun))
  (set `/Game/VR_Weapons/Global/Blueprints/BP_Gun.Bipod` self _output_get)
  (set `/Game/VR_Weapons/Global/Blueprints/BP_Gun.Weapon mounted` true _output_get)
  (add `/Game/VR_Weapons/Global/Blueprints/BP_Gun.Weapon fired` _output_get (`|CreateDelegate` :!event `Animate recoil`))
  (add `/Game/VR_Weapons/Global/Blueprints/BP_Gun.Weapon released while mounted` _output_get (`|CreateDelegate` :!event `Gun released while mounted`))
  (`SceneComponent.K2_AttachToComponent` (`self.Pivot`) (`self.Turret pivot`) "None" "KeepWorld" "KeepWorld" "KeepWorld" true))

(fn `Range before detaching`
  (params (`Slider Rail Position` :type "Float (double-precision)"))
  (returns (ReturnValue :type Boolean))
  (return false) ; stop gun detaching
)

(fn `Update mounted weapon transform`
  (bind (_mounted_gun_relative_rotation_roll _mounted_gun_relative_rotation_pitch _mounted_gun_relative_rotation_yaw) (`KismetMathLibrary.BreakRotator` (`self.Mounted Gun Relative Rotation`)))
  (`SceneComponent.K2_SetRelativeRotation` (`self.Pivot`) (`KismetMathLibrary.MakeRotator` 0.0 _mounted_gun_relative_rotation_pitch) false false) ; rotate pivot left/right
  (`SceneComponent.K2_SetRelativeRotation` (`self.Turret pivot`) (`KismetMathLibrary.MakeRotator` 0.0 0.0 _mounted_gun_relative_rotation_yaw) false false) ; rotate slider rail up/down
  (if (`self.Use slider rail`)
    (`SceneComponent.K2_SetRelativeLocation` (`self.Slider Rail dummy`) (`KismetMathLibrary.MakeVector` (`KismetMathLibrary.FClamp` (`self.MountedGunPosition`) -15.0 4.0)) false false)))

(fn `UserConstructionScript`
  (`parent.UserConstructionScript`))