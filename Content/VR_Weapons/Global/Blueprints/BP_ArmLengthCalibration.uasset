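; BP_ArmLengthCalibration is a VR calibration station that shows where to stand and gives feedback during arm-length calibration.
; Entering its overlap box tints the StandHere and CTA texts orange, and leaving restores white, hides the Complete text and shows the CTA again.
; The ArmLengthCalibrated function swaps the CTA for the Complete text; the measurement itself is not done in this Blueprint.
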(event `self.Overlap box.OnComponentBeginOverlap`
  (params (OverlappedComponent :type "PrimitiveComponent Object Reference") (OtherActor :type "Actor Object Reference") (OtherComp :type "PrimitiveComponent Object Reference") (OtherBodyIndex :type Integer) (bFromSweep :type Boolean) (SweepResult :type "HitResult Structure (by ref)"))
  (`TextRenderComponent.SetTextRenderColor` (`self.Stand here`) (`KismetMathLibrary.Conv_LinearColorToColor` (struct :`R` 1.0 :`G` 0.274507 :`A` 1.0)))
  (`TextRenderComponent.SetTextRenderColor` (`self.CTA`) (`KismetMathLibrary.Conv_LinearColorToColor` (struct :`R` 1.0 :`G` 0.274507 :`A` 1.0))))

(event `self.Overlap box.OnComponentEndOverlap`
  (params (OverlappedComponent :type "PrimitiveComponent Object Reference") (OtherActor :type "Actor Object Reference") (OtherComp :type "PrimitiveComponent Object Reference") (OtherBodyIndex :type Integer))
  (`TextRenderComponent.SetTextRenderColor` (`self.Stand here`) (`KismetMathLibrary.Conv_LinearColorToColor` (struct :`R` 1.0 :`G` 1.0 :`B` 1.0 :`A` 1.0)))
  (`TextRenderComponent.SetTextRenderColor` (`self.CTA`) (`KismetMathLibrary.Conv_LinearColorToColor` (struct :`R` 1.0 :`G` 1.0 :`B` 1.0 :`A` 1.0)))
  (`SceneComponent.SetVisibility` (`self.Complete`) false false)
  (`SceneComponent.SetVisibility` (`self.CTA`) true false))

(fn `Arm length calibrated`
  (`SceneComponent.SetVisibility` (`self.Complete`) true false)
  (`SceneComponent.SetVisibility` (`self.CTA`) false false))

(fn `UserConstructionScript`)