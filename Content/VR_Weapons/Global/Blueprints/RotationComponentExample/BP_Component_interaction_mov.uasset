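; Example VR interaction actor with a mesh the player grabs with a motion controller and slides along a single chosen axis.
; Pickup stores the hand position in mesh-local space, then Tick asks BPCComponentInteraction for the target offset and moves the mesh only while inside the min and max limits.
; The same component drives impact vibration and a bolt-click sound from the clamped value.
; Dropping or the controller leaving the box releases it.
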(event `self.ReceiveBeginPlay`
  (bind _outactors (`GameplayStatics.GetAllActorsOfClass` "/Game/VR_Weapons/Global/Blueprints/RotationComponentExample/Tester.Tester_C"))
  (set `self.Tester` (`|GetArrayItem` _outactors)))

(event `self.ReceiveTick`
  (params (DeltaSeconds :type "Float (single-precision)"))
  (bind _mesh (`self.Mesh`))
  (if (`self.Grabbed`)
    (bind _distance (`/Game/VR_Weapons/Global/Blueprints/BPC_ComponentInteraction.Move component using target` (`self.BPC_ComponentInteraction`) (`/Game/VR_Weapons/Pawn/Blueprints/BP_MotionController.GrabSphere` (`self.MotionController`)) self (`self.Axis`) (`self.grab position`)))
    (`/Game/VR_Weapons/Global/Blueprints/BPC_ComponentInteraction.Component impact vibration and sound` (`self.BPC_ComponentInteraction`) (`self.MotionController`) (`self.Min location`) (`self.Max location`) (`KismetMathLibrary.FClamp` _distance (`self.Min location`) (`self.Max location`)) 0.6 false "/Game/VR_Weapons/Global/Audio/Bolt_click_Cue.Bolt_click_Cue")
    (if (and (> _distance (`self.Min location`)) (< _distance (`self.Max location`)))
      (switch `/Game/VR_Weapons/Global/Blueprints/ComponentMovementAxis` (`self.Axis`)
        (:`NewEnumerator0`
          (`SceneComponent.K2_SetRelativeLocation` _mesh (`KismetMathLibrary.MakeVector` _distance) false false))
        (:`NewEnumerator1`
          (`SceneComponent.K2_SetRelativeLocation` _mesh (`KismetMathLibrary.MakeVector` 0.0 _distance) false false))
        (:`NewEnumerator2`
          (`SceneComponent.K2_SetRelativeLocation` _mesh (`KismetMathLibrary.MakeVector` 0.0 0.0 _distance) false false))))))

(event `/Game/VR_Weapons/Global/Blueprints/BPI_pickup.Drop actor`
  (set `self.Grabbed` false :!label _label)
  (set `self.MotionController` null)
  (`KismetSystemLibrary.PrintString` "RELEASED" true true (struct :`G` 0.66 :`B` 1.0 :`A` 1.0) 1.0))

(event `self.Box.OnComponentEndOverlap`
  (params (OverlappedComponent :type "PrimitiveComponent Object Reference") (OtherActor :type "Actor Object Reference") (OtherComp :type "PrimitiveComponent Object Reference") (OtherBodyIndex :type Integer))
  (if (== OtherActor (`self.MotionController`))
    (goto _label)))

(fn `Measure grab distance`
  (set `self.grab position` (`KismetMathLibrary.InverseTransformLocation` (`SceneComponent.K2_GetComponentToWorld` (`self.Mesh`)) (`SceneComponent.K2_GetComponentLocation` (`/Game/VR_Weapons/Pawn/Blueprints/BP_MotionController.GrabSphere` (`self.MotionController`))))))

(fn `Pickup actor`
  (params (Hand :type "EControllerHand Enum" :default "Left") (`Grip or grab` :type "/Game/VR_Weapons/Pawn/Blueprints/E_GrabType Enum" :default "NewEnumerator1") (`Motion Controller Actor` :type "/Game/VR_Weapons/Pawn/Blueprints/BP_MotionController Object Reference") (AttachTo :type "SceneComponent Object Reference"))
  (returns (WeaponType :type "/Game/VR_Weapons/Pawn/Blueprints/E_WeaponType Enum") (GunGrabbed :type Boolean))
  (set `self.MotionController` `Motion Controller Actor`)
  (`self.Measure grab distance`)
  (set `self.Grabbed` true)
  (return "NewEnumerator0" false))

(fn `UserConstructionScript`)