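; Example VR interactable actor whose mesh rotates around a selected axis to follow the grabbing motion controller, or a Tester actor that overlaps its box.
; While grabbed, Tick gets an angle from the component interaction helper and applies it only within the min/max limits.
; The helper also drives impact vibration and sound from the clamped angle.
; Dropping, or the controller leaving the box, releases the grab.
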(event `self.ReceiveBeginPlay`
  (bind _outactors (`GameplayStatics.GetAllActorsOfClass` "/Game/VR_Weapons/Global/Blueprints/RotationComponentExample/Tester.Tester_C"))
  (set `self.Tester` (`|GetArrayItem` _outactors)))

(event `self.ReceiveTick`
  (params (DeltaSeconds :type "Float (single-precision)"))
  (bind _debug (`self.debug`))
  (bind _mesh (`self.Mesh`))
  (if (`self.Grabbed`)
    (bind _rotation (`/Game/VR_Weapons/Global/Blueprints/BPC_ComponentInteraction.Rotate component using target` (`self.BPC_ComponentInteraction`) (`self.Axis`) (select `bool` (`self.Use tester`) :`false` (`/Game/VR_Weapons/Pawn/Blueprints/BP_MotionController.GrabSphere` (`self.MotionController`)) :`true` (`/Game/VR_Weapons/Global/Blueprints/RotationComponentExample/Tester.Sphere` (`self.Tester`)) :!type "SceneComponent Object Reference") (`self.Mesh`) (`self.Offset`)))
    (`KismetSystemLibrary.PrintString` (`KismetStringLibrary.Conv_DoubleToString` _rotation) _debug _debug (struct :`G` 1.0 :`B` 0.004862 :`A` 1.0) 0.0)
    (`/Game/VR_Weapons/Global/Blueprints/BPC_ComponentInteraction.Component impact vibration and sound` (`self.BPC_ComponentInteraction`) (`self.MotionController`) (`self.Min rotation`) (`self.Max rotation`) (`KismetMathLibrary.FClamp` _rotation (`self.Min rotation`) (`self.Max rotation`)) 0.6 false "/Game/VR_Weapons/Global/Audio/Bolt_click_Cue.Bolt_click_Cue")
    (if (and (> _rotation (`self.Min rotation`)) (< _rotation (`self.Max rotation`)))
      (switch `/Game/VR_Weapons/Global/Blueprints/ComponentRotationAxis` (`self.Axis`)
        (:`NewEnumerator0`
          (`SceneComponent.K2_SetRelativeRotation` _mesh (`KismetMathLibrary.MakeRotator` _rotation) false false))
        (:`NewEnumerator1`
          (`SceneComponent.K2_SetRelativeRotation` _mesh (`KismetMathLibrary.MakeRotator` 0.0 _rotation) false false))
        (:`NewEnumerator2`
          (`SceneComponent.K2_SetRelativeRotation` _mesh (`KismetMathLibrary.MakeRotator` 0.0 0.0 _rotation) false false))))))

(event `/Game/VR_Weapons/Global/Blueprints/BPI_pickup.Drop actor`
  (set `self.Grabbed` false :!label _label)
  (set `self.MotionController` null)
  (`KismetSystemLibrary.PrintString` "RELEASED" true true (struct :`G` 0.66 :`B` 1.0 :`A` 1.0) 1.0))

(event `self.Box.OnComponentEndOverlap`
  (params (OverlappedComponent :type "PrimitiveComponent Object Reference") (OtherActor :type "Actor Object Reference") (OtherComp :type "PrimitiveComponent Object Reference") (OtherBodyIndex :type Integer))
  (if (== OtherActor (`self.MotionController`))
    (goto _label)
    (elif (== OtherActor (`self.Tester`))
      (set `self.Grabbed` false))))

(event `self.Box.OnComponentBeginOverlap`
  (params (OverlappedComponent :type "PrimitiveComponent Object Reference") (OtherActor :type "Actor Object Reference") (OtherComp :type "PrimitiveComponent Object Reference") (OtherBodyIndex :type Integer) (bFromSweep :type Boolean) (SweepResult :type "HitResult Structure (by ref)"))
  (if (== OtherActor (`self.Tester`))
    (set `self.Grabbed` true)
    (set `self.Use tester` true)))

(fn `Pickup actor`
  (params (Hand :type "EControllerHand Enum" :default "Left") (`Grip or grab` :type "/Game/VR_Weapons/Pawn/Blueprints/E_GrabType Enum" :default "NewEnumerator1") (`Motion Controller Actor` :type "/Game/VR_Weapons/Pawn/Blueprints/BP_MotionController Object Reference") (AttachTo :type "SceneComponent Object Reference"))
  (returns (WeaponType :type "/Game/VR_Weapons/Pawn/Blueprints/E_WeaponType Enum") (GunGrabbed :type Boolean))
  (set `self.MotionController` `Motion Controller Actor`)
  (set `self.Grabbed` true)
  (return "NewEnumerator0" false))

(fn `UserConstructionScript`)