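; Blueprint component for interactive VR weapon parts, turning a hand or target position into part movement and impact feedback.
; Helper functions convert the target into owner or gun local space, returning a look-at roll, pitch or yaw angle, or single-axis travel from a start location.
; An impact event fires controller rumble and sound once upon reaching either movement limit, using flip-flopped previous-frame values to estimate speed for scaling and re-arming.
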(event `Component impact vibration and sound`
  (params (MotionController :type "/Game/VR_Weapons/Pawn/Blueprints/BP_MotionController Object Reference") (`Min rotation/movement` :type "Float (double-precision)") (`Max rotation/movement` :type "Float (double-precision)") (`Current rotation/movement` :type "Float (double-precision)") (`Vibration intensity` :type "Float (double-precision)" :default 0.6) (`Use velocity to scale vibration intensity` :type Boolean :default true) (`Impact sound` :type "SoundBase Object Reference"))
  (`self.Component impact vibration/sound` MotionController `Min rotation/movement` `Max rotation/movement` `Current rotation/movement` `Vibration intensity` `Use velocity to scale vibration intensity` `Impact sound`))

(fn `Move component using target`
  (params (Target :type "SceneComponent Object Reference") (Actor :type "Actor Object Reference") (Axis :type "/Game/VR_Weapons/Global/Blueprints/ComponentMovementAxis Enum" :default "NewEnumerator0") (`Component start location` :type "Vector Structure"))
  (returns (Distance :type "Float (double-precision)"))
  ;[0 0 0] function for rotating components
  (return (- (select `/Game/VR_Weapons/Global/Blueprints/ComponentMovementAxis` Axis :`NewEnumerator0` (.x (`KismetMathLibrary.InverseTransformLocation` (`Actor.GetTransform` Actor) (`SceneComponent.K2_GetComponentLocation` Target))) :`NewEnumerator1` (.y (`KismetMathLibrary.InverseTransformLocation` (`Actor.GetTransform` Actor) (`SceneComponent.K2_GetComponentLocation` Target))) :`NewEnumerator2` (.z (`KismetMathLibrary.InverseTransformLocation` (`Actor.GetTransform` Actor) (`SceneComponent.K2_GetComponentLocation` Target)))) (select `/Game/VR_Weapons/Global/Blueprints/ComponentMovementAxis` Axis :`NewEnumerator0` (.x `Component start location`) :`NewEnumerator1` (.y `Component start location`) :`NewEnumerator2` (.z `Component start location`)))))

(fn `Rotate component using target`
  (params (Selection :type "/Game/VR_Weapons/Global/Blueprints/ComponentRotationAxis Enum" :default "NewEnumerator0") (Target :type "SceneComponent Object Reference") (`Component to rotate` :type "SceneComponent Object Reference") (offset :type "Float (double-precision)"))
  (returns (Rotation :type "Float (double-precision)"))
  (bind _pitch (.pitch (`KismetMathLibrary.FindLookAtRotation` (* (`SceneComponent.RelativeLocation` (`local.Component to rotate`)) (1.0 0.0 1.0)) (* (`KismetMathLibrary.InverseTransformLocation` (`Actor.GetTransform` (`self.GetOwner`)) (`SceneComponent.K2_GetComponentLocation` (`local.Target`))) (1.0 0.0 1.0)))))
  (bind _yaw (.yaw (`KismetMathLibrary.FindLookAtRotation` (* (`SceneComponent.RelativeLocation` (`local.Component to rotate`)) (1.0 0.0 1.0)) (* (`KismetMathLibrary.InverseTransformLocation` (`Actor.GetTransform` (`self.GetOwner`)) (`SceneComponent.K2_GetComponentLocation` (`local.Target`))) (1.0 0.0 1.0)))))
  (bind _pitch_2 (.pitch (`KismetMathLibrary.FindLookAtRotation` (* (`KismetMathLibrary.InverseTransformLocation` (`Actor.GetTransform` (`self.GetOwner`)) (`SceneComponent.K2_GetComponentLocation` (`local.Target`))) (0.0 1.0 1.0)) (* (`SceneComponent.RelativeLocation` (`local.Component to rotate`)) (0.0 1.0 1.0)))))
  ;[0 0 0] function for rotating components
  (switch `/Game/VR_Weapons/Global/Blueprints/ComponentRotationAxis` Selection
    (:`NewEnumerator0`
      ;[1 1 1] Roll
      (return (+ (`KismetMathLibrary.SelectFloat` (- 180.0 _pitch_2) _pitch_2 (> (.yaw (`KismetMathLibrary.FindLookAtRotation` (* (`KismetMathLibrary.InverseTransformLocation` (`Actor.GetTransform` (`self.GetOwner`)) (`SceneComponent.K2_GetComponentLocation` (`local.Target`))) (0.0 1.0 1.0)) (* (`SceneComponent.RelativeLocation` (`local.Component to rotate`)) (0.0 1.0 1.0)))) 0.0)) (`local.offset`))))
    (:`NewEnumerator1`
      ;[1 1 1] Pitch
      (`KismetSystemLibrary.PrintString` (`KismetStringLibrary.Conv_DoubleToString` _yaw) true true (struct :`G` 0.66 :`B` 1.0 :`A` 1.0) 0.0)
      (return (+ (`KismetMathLibrary.SelectFloat` (- 180.0 _pitch) _pitch (!= _yaw 0.0)) (`local.offset`))))
    (:`NewEnumerator2`
      ;[1 1 1] Yaw
      (return (+ (.yaw (`KismetMathLibrary.FindLookAtRotation` (* (`SceneComponent.RelativeLocation` (`local.Component to rotate`)) (1.0 1.0 0.0)) (* (`KismetMathLibrary.InverseTransformLocation` (`Actor.GetTransform` (`self.GetOwner`)) (`SceneComponent.K2_GetComponentLocation` (`local.Target`))) (1.0 1.0 0.0)))) (`local.offset`))))))