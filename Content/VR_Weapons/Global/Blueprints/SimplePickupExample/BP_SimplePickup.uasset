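; Example VR pickup actor that motion controller hands can grab, hold and throw, with multiplayer replication.
; PickupActor switches the hand to a single animation, attaches the mesh locally at an offset, and requests ownership through the pawn.
; Replicate polls until an owner check passes, then calls ServerAttach; absolute scale prevents left-hand flipping.
; DropActor restores the hand AnimBP, re-enables physics, and replicates the throw velocity before clearing ownership.
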(event `Replicate`
  (if (!= (`self.GetOwner`) null) :!label _label
    (`self.Server attach` (`self.HandMesh`))
    (else
      (`KismetSystemLibrary.Delay` 0.1)
      (goto _label))))

(event `Server attach`
  (params (HandMesh :type "SkeletalMeshComponent Object Reference"))
  (set `self.HandMesh` HandMesh)
  (`self.Attach`))

(event `/Game/VR_Weapons/Global/Blueprints/BPI_pickup.Drop actor`
  (bind _mesh (`self.Mesh`))
  (`SkeletalMeshComponent.SetAnimationMode` (`self.HandMesh`) "AnimationBlueprint" true)
  (set `self.HandMesh` null)
  (`self.K2_DetachFromActor` "KeepWorld" "KeepWorld" "KeepWorld")
  (`PrimitiveComponent.SetSimulatePhysics` _mesh true)
  (`self.Server drop` (`SceneComponent.GetComponentVelocity` _mesh)))

(event `Server drop`
  (params (Impulse :type "Vector Structure"))
  (`/Game/VR_Weapons/Networking/Networking.Replicate actor throwing` (`self.Networking`) (`self.Mesh`) Impulse)
  (`self.SetOwner` null))

(fn `Attach`
  (bind _mesh (`self.Mesh`))
  (bind _attach_offset (`self.Attach offset`))
  (`PrimitiveComponent.SetSimulatePhysics` (`self.Mesh`) false)
  (`SceneComponent.K2_AttachToComponent` (`self.Mesh`) (`self.HandMesh`) "None" "SnapToTarget" "SnapToTarget" "KeepWorld" false)
  (`SceneComponent.K2_SetRelativeTransform` _mesh _attach_offset false false)
  (`SceneComponent.SetWorldScale3D` _mesh (`KismetMathLibrary.Vector_GetAbs` (.scale _attach_offset))) ; Stop flipping in left hand
)

(fn `Pickup actor`
  (params (Hand :type "EControllerHand Enum" :default "Left") (`Grip or grab` :type "/Game/VR_Weapons/Pawn/Blueprints/E_GrabType Enum" :default "NewEnumerator1") (`Motion Controller Actor` :type "/Game/VR_Weapons/Pawn/Blueprints/BP_MotionController Object Reference") (AttachTo :type "SceneComponent Object Reference"))
  (returns (WeaponType :type "/Game/VR_Weapons/Pawn/Blueprints/E_WeaponType Enum") (GunGrabbed :type Boolean))
  (`SkeletalMeshComponent.SetAnimationMode` (`self.HandMesh`) "AnimationBlueprint" true) ; 5.4 fix: Reset existing hand if already grabbed by other hand
  (bind _output_get (set `self.HandMesh` (`/Game/VR_Weapons/Pawn/Blueprints/BP_MotionController.HandMesh` `Motion Controller Actor`)))
  ;[0 0 0] Set hand animation
  (`self.Set animation` _output_get)
  ;[0 0 0] Set owner
  (bind _asmotion_controller_pawn (cast `/Game/VR_Weapons/Pawn/Blueprints/MotionControllerPawn` (`GameplayStatics.GetPlayerPawn` 0)))
  (`/Game/VR_Weapons/Pawn/Blueprints/MotionControllerPawn.Server set actor owner in pawn` _asmotion_controller_pawn self)
  ;[0 0 0] Attach locally
  (`self.Attach`)
  (`self.Replicate`)
  (return "NewEnumerator0" false))

(fn `Set animation`
  (params (Hand :type "SkeletalMeshComponent Object Reference"))
  (bind _anim_animtoplay (break `SingleAnimationPlayData` (`self.Anim`)))
  (`SkeletalMeshComponent.SetAnimationMode` Hand "AnimationSingleNode" true)
  (`SkeletalMeshComponent.SetAnimation` Hand _anim_animtoplay))

(fn `UserConstructionScript`)