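; Networked VR bipod/aiming stand that mounts a gun and lets the holding hand aim it.
; On Tick, the local client turns controller position into pivot rotation and slider offset, sent to the server.
; Pulling the slider beyond its range detaches the gun back to the hand with haptics.
; A fire-rate-scaled recoil timeline is multicast, and a dummy hand replaces the controller hand mesh for non-IK setups.
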(event `self.ReceiveBeginPlay`
  ;[1 0.6016 0] Remove dummy mesh
  (`ActorComponent.K2_DestroyComponent` (`self.Dummy_mounted_weapon`)) ; remove dummy weapon
  (set `/Game/VR_Weapons/Networking/Networking.Debug network settings` (`self.Debug`) (`self.Networking`)))

(event `Server animate recoil`
  ;[0.494 0.3303 1] Replicate recoil on server
  (`self.Multicast animate recoil`))

(event `Multicast animate recoil`
  (bind _aiming_stand_location (`self.Aiming stand location`))
  ;[0.494 0.3303 1] Replicate recoil on server
  (if (not (`self.Locally controlled`))
    ;[0 0 0] Recoil
    (`TimelineComponent.SetPlayRate` (`self.Bipod recoil`) (/ 1.0 (* (`/Game/VR_Weapons/Global/Blueprints/BP_Gun.Automatic firing rate` (`self.BP gun`)) 10.0)) :!label _label) ; 2.2 update: use weapon's firing rate to control duration of bipod recoil movement \n(can be useful for machine guns)
    (set `self.Aiming stand location` (`self.K2_GetActorLocation`))
    (bind (_direction _bipod _slider_rail) (`Timeline|Bipod recoil` :!via `PlayFromStart`)
      (:`Update`
        (`self.K2_SetActorLocation` (`KismetMathLibrary.VLerp` _aiming_stand_location (+ _aiming_stand_location (* (`SceneComponent.GetForwardVector` (`self.Pivot`)) (`self.Recoil movement multiplier`))) _bipod))
        (set `self.Slider rail offset` _slider_rail)))))

(event `Animate recoil`
  ;[0 0 0] Recoil
  ;;[0.494 0.3303 1] Replicate recoil on server
  (`self.Server animate recoil`)
  (goto _label))

(event `Server update weapon position`
  (params (MountedGunRotation :type "Rotator Structure") (MountedGunPosition :type "Float (double-precision)"))
  ;[0 0 0] Update gun position by rotating the pivot and moving the slider rail
  ; (calculated by measuring Look at Rotation and distance between motion controller and pivot)
  ;;[0.494 0.3303 1] Update mounted weapon transform on server
  (set `self.Mounted Gun Relative Rotation` MountedGunRotation)
  (set `self.MountedGunPosition` MountedGunPosition))

(event `self.ReceiveTick`
  (params (DeltaSeconds :type "Float (single-precision)"))
  (bind _debug (`self.Debug`))
  (bind _bp_gun (`self.BP gun`))
  ;[0 0 0] Update gun position by rotating the pivot and moving the slider rail
  ; (calculated by measuring Look at Rotation and distance between motion controller and pivot)
  (`/Engine/EditorBlueprintResources/StandardMacros.IsValid` (`self.MotionController`)
    (:`Is Valid`
      (`|ExecutionSequence`
        (:`then_0`
          (if (`self.Locally controlled`)
            (`KismetSystemLibrary.PrintString` "Updating pivot" true true (struct :`R` 0.019638 :`G` 0.119792 :`B` 0.068515 :`A` 1.0) 0.0)
            (switch `/Game/VR_Weapons/Pawn/Blueprints/E_GripEnum` (`/Game/VR_Weapons/Pawn/Blueprints/BP_MotionController.GripState` (`self.MotionControllerBP`))
              (:`NewEnumerator2`
                _)
              (:`NewEnumerator4`
                _))
            (`self.Update Pivot rotation`)
            (bind _slider_rail_x_pos (`self.Update Slider Rail Position`))
            (`KismetSystemLibrary.PrintString` (`KismetStringLibrary.Concat_StrStr` "Pivot rotation: " (`KismetStringLibrary.Conv_RotatorToString` (`self.Mounted Gun Relative Rotation`))) true true (struct :`G` 0.66 :`B` 1.0 :`A` 1.0) 0.0)
            (`self.Server update weapon position` (`self.Mounted Gun Relative Rotation`) (`self.MountedGunPosition`))
            (if (`self.Range before detaching` _slider_rail_x_pos)
              (`self.Haptics`)
              ;[0.494 0.3303 1] Update all clients when gun has been removed
              (`self.Server remove from bipod`)
              ;[0.494 0.3303 1] 2.2.1 remove instantly and attach to local player's hand
              (bind _returnvalue (`SceneComponent.K2_AttachToComponent` (`self.K2_GetRootComponent` _bp_gun) (`/Game/VR_Weapons/Pawn/Blueprints/BP_MotionController.HandMesh` (`self.MotionControllerBP`)) (`/Game/VR_Weapons/Global/Blueprints/BP_Gun.Primary hand attach socket` _bp_gun) "SnapToTarget" "SnapToTarget" "SnapToTarget" false)) ; re-attach gun to hand when unmounted
              (`KismetSystemLibrary.PrintString` (`KismetStringLibrary.Concat_StrStr` "Pickup = " (`KismetStringLibrary.Conv_BoolToString` _returnvalue)) _debug _debug (struct :`G` 0.66 :`B` 1.0 :`A` 1.0) 6.0)
              (`/Game/VR_Weapons/Global/Blueprints/BP_Gun.Left/Right hand gripping` (`self.BP gun`))
              (`self.Gun removed from bipod`))))
        (:`then_1`
          (`self.Update mounted weapon transform`) ; 2.2 update
          (if (`self.Debug`)
            (`KismetSystemLibrary.DrawDebugString` (+ (`SceneComponent.K2_GetComponentLocation` (`self.Pivot`)) (0.0 0.0 10.0)) (`KismetStringLibrary.Concat_StrStr` "Pivot rotation: " (`KismetStringLibrary.Conv_RotatorToString` (`self.Mounted Gun Relative Rotation`))) null (struct :`R` 1.0 :`G` 0.146251 :`A` 1.0))
            (`KismetSystemLibrary.DrawDebugString` (+ (`SceneComponent.K2_GetComponentLocation` (`self.Slider Rail dummy`)) (0.0 0.0 5.0)) (`KismetStringLibrary.Concat_StrStr` "MountedGunPosition: " (`KismetStringLibrary.Conv_DoubleToString` (`self.MountedGunPosition`))) null (struct :`R` 1.0 :`G` 0.080133 :`A` 1.0))))))))

(event `Server remove from bipod`
  ;[0.494 0.3303 1] Update all clients when gun has been removed
  (set `self.Mounted` false)
  (`self.Gun removed from bipod`) ; 2.2.1 remove on server
)

(fn `Grab gun while mounted`
  (params (Hand :type "EControllerHand Enum" :default "Left"))
  (bind _debug (`self.Debug`))
  (bind _primary_motion_controller_bp (`/Game/VR_Weapons/Global/Blueprints/BP_Gun.Primary Motion Controller BP` (`self.BP gun`)))
  (`KismetSystemLibrary.PrintString` "Grabbing gun while mounted" _debug _debug (struct :`G` 1.0 :`B` 0.05424 :`A` 1.0) 5.0)
  (`/Game/VR_Weapons/Global/Blueprints/BP_Gun.Select Dummy Hand Orientation` (`self.BP gun`))
  (`self.Show/hide dummy hand` false) ; Hide motion controller hand mesh and show fake hand mesh
  (set `self.MotionControllerBP` _primary_motion_controller_bp) ; Set motion controller actor reference
  (bind _output_get (set `self.MotionController` (`/Game/VR_Weapons/Pawn/Blueprints/BP_MotionController.MotionController` _primary_motion_controller_bp))) ; Set motion controller component  reference
  (set `self.Starting distance` (`KismetMathLibrary.Vector_Distance` (`SceneComponent.K2_GetComponentLocation` _output_get) (`SceneComponent.K2_GetComponentLocation` (`self.Slider Rail dummy`)))) ; Use this as a starting point to measure the motion controller movement
  (`self.SetActorScale3D` (`self.BP gun`) (1.0 1.0 1.0)) ; 2.2.1 ensure correct orientation if left hand is grabbing
)

(fn `Gun released while mounted`
  (`self.Set Is Locally Controlled` false))

(fn `Mount gun`
  (bind _bp_gun (`self.BP gun`))
  (bind _debug (`self.Debug`))
  (bind _debug_2 (`self.Debug`))
  (bind _primary_motion_controller_bp (`/Game/VR_Weapons/Global/Blueprints/BP_Gun.Primary Motion Controller BP` _bp_gun))
  ;[0 0 0] Check gun has not already been mounted
  (if (not (`self.Mounted`))
    (set `self.Mounted` true)
    ;[0 0 0] Set slider rail start position
    (`SceneComponent.K2_SetRelativeLocation` (`self.Slider Rail dummy`) (`KismetMathLibrary.MakeVector` (`KismetMathLibrary.Vector_Distance2D` (`SceneComponent.K2_GetComponentLocation` (`self.Slider Rail dummy`)) (`SceneComponent.GetSocketLocation` (`/Game/VR_Weapons/Global/Blueprints/BP_Gun.Gun mesh` (`self.BP gun`)) "Bipod"))) false false) ; set slider rail position so its underneath the gun's "bipod" socket
    ;[0 0 0] Attach gun to bipod
    (`self.K2_AttachToComponent` (`self.BP gun`) (`self.Attach dummy`) "None" "SnapToTarget" "SnapToTarget" "KeepRelative" true) ; Attach gun to the "Attach dummy". \n\nThis positions the gun correctly on the bipod. \n\nThe Attach dummy is attached to the Slider rail and Pivot \nso the gun can be moved forward/back and rotated in all directions
    (`KismetSystemLibrary.PrintString` "Mounted" _debug _debug (struct :`R` 0.003254 :`G` 1.0 :`A` 1.0) 3.0)
    (`self.SetActorScale3D` (`self.BP gun`) (1.0 1.0 1.0)) ; Ensure correct orientation if left hand is grabbing
    (`self.SetOwner` (`self.GetOwner` _bp_gun))
    (`|ExecutionSequence`
      (:`then_0`
        (`self.Show/hide dummy hand` false) ; Hide motion controller hand mesh and show fake hand mesh
        (bind _output_get (set `self.MotionController` (`/Game/VR_Weapons/Pawn/Blueprints/BP_MotionController.MotionController` _primary_motion_controller_bp))) ; Set motion controller component  reference
        (set `self.Starting distance` (`KismetMathLibrary.Vector_Distance` (`SceneComponent.K2_GetComponentLocation` _output_get) (`SceneComponent.K2_GetComponentLocation` (`self.Slider Rail dummy`)))) ; Use this as a starting point to measure the motion controller movement
        (`/Game/VR_Weapons/Global/Blueprints/BP_Gun.Select Dummy Hand Orientation` (`self.BP gun`))
        (`self.Haptics`)
        (add `/Game/VR_Weapons/Global/Blueprints/BP_Gun.Weapon released while mounted` (`self.BP gun`) (`|CreateDelegate` :!event `Gun released while mounted`)) ; 2.2 update
      )
      (:`then_1`
        (set `self.MotionControllerBP` _primary_motion_controller_bp) ; Set motion controller actor reference
      ))
    (else
      (`KismetSystemLibrary.PrintString` "Already mounted" _debug_2 _debug_2 (struct :`R` 1.0 :`G` 0.354956 :`A` 1.0)))))

(fn `OnRep_Mounted`
  (bind _debug (`self.Debug`))
  (bind _bp_gun (`self.BP gun`))
  (if (not (`self.Mounted`))
    (set `self.Starting distance` 0.0)
    (set `self.MountedGunPosition` 0.0)
    (`/Engine/EditorBlueprintResources/ActorMacros.Switch Has Authority` ; 2.2.1 only attach if server
      (:`Authority`
        (bind _returnvalue (`SceneComponent.K2_AttachToComponent` (`self.K2_GetRootComponent` _bp_gun) (`/Game/VR_Weapons/Pawn/Blueprints/BP_MotionController.HandMesh` (`self.MotionControllerBP`)) (`/Game/VR_Weapons/Global/Blueprints/BP_Gun.Primary hand attach socket` _bp_gun) "SnapToTarget" "SnapToTarget" "SnapToTarget" false)) ; re-attach gun to hand when unmounted
        (`KismetSystemLibrary.PrintString` (`KismetStringLibrary.Concat_StrStr` "Pickup = " (`KismetStringLibrary.Conv_BoolToString` _returnvalue)) _debug _debug (struct :`G` 0.66 :`B` 1.0 :`A` 1.0) 6.0)
        (`/Game/VR_Weapons/Global/Blueprints/BP_Gun.Left/Right hand gripping` (`self.BP gun`)))
      (:`Remote`
        _))
    (`self.Show/hide dummy hand` true) ; Show motion controller hand mesh and hide fake hand mesh
  ))

(fn `Range before detaching`
  (params (`Slider Rail Position` :type "Float (double-precision)"))
  (returns (ReturnValue :type Boolean))
  (return (and (or (< `Slider Rail Position` (`self.Min distance for detach`)) (> `Slider Rail Position` (`self.Max distance for detach`))) (`self.Mounted`))))

(fn `Set Is Locally Controlled`
  (params (`Locally controlled` :type Boolean))
  (bind _output_get (set `self.Locally controlled` `Locally controlled`))
  (if (not _output_get)
    (set `self.MotionController` null) ; clear reference when user releases grip
  ))

(fn `Show/hide dummy hand`
  (params (`Hand visibility` :type Boolean))
  ;[0 0 0] Hides BP motion controller hand mesh. Then shows fake hand attached to rifle. This prevents the real hand mesh from rotating the wrong way and shows the hand mesh as always being aligned to the gun's pistol grip
  (if (and (`KismetSystemLibrary.IsValid` (`self.MotionControllerBP`)) (not (`/Game/VR_Weapons/Global/Blueprints/BP_Gun.Pawn owner using IK body` (`self.BP gun`))))
    (`SceneComponent.SetVisibility` (`/Game/VR_Weapons/Pawn/Blueprints/BP_MotionController.HandMesh` (`self.MotionControllerBP`)) `Hand visibility` false) ; Hide/show real motion controller mesh
    (`/Game/VR_Weapons/Global/Blueprints/BP_Gun.Toggle mounted gun dummy hand visibility` (`self.BP gun`) (not `Hand visibility`)) ; 2.2 update: This function now supports \nany weapon type that can be mounted
  ))

(fn `Update mounted weapon transform`
  (`SceneComponent.K2_SetRelativeRotation` (`self.Pivot`) (`self.Mounted Gun Relative Rotation`) false false) ; 2.2 update: now uses relative rotation (to support different rotations for child components)
  (`SceneComponent.K2_SetRelativeLocation` (`self.Slider Rail dummy`) (`KismetMathLibrary.MakeVector` (`self.MountedGunPosition`)) false false))

(fn `Update Pivot rotation`
  (locals (Offset :type "Vector Structure" :default (0.0 0.0 2.0)))
  (set `self.Mounted Gun Relative Rotation` (`KismetMathLibrary.FindLookAtRotation` (+ (`KismetMathLibrary.InverseTransformLocation` (`self.GetTransform`) (`SceneComponent.K2_GetComponentLocation` (`self.MotionController`))) (`local.Offset`)) (`SceneComponent.RelativeLocation` (`self.Pivot`)))))

(fn `Update Slider Rail Position`
  (returns (`Slider rail x pos` :type "Float (double-precision)"))
  (bind _returnvalue (- (`self.Starting distance`) (`KismetMathLibrary.Vector_Distance` (`SceneComponent.K2_GetComponentLocation` (`self.MotionController`)) (`SceneComponent.K2_GetComponentLocation` (`self.Pivot`)))))
  (set `self.MountedGunPosition` (- _returnvalue (`self.Slider rail offset`)))
  (return _returnvalue))

(fn `UserConstructionScript`)