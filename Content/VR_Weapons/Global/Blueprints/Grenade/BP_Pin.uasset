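; VR grenade pin actor that is removed by hand or teeth, flagging its parent grenade as ready to explode on release.
; Pickup requires a held grenade, then attaches the pin to the hand socket with haptics and updates the server.
; Leaving overlap with a Teeth-tagged component also removes the pin and drops it.
; Dropping detaches it with physics, propagates to non-local clients, and starts a timed destroy.
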(event `self.Overlap.OnComponentBeginOverlap`
  (params (OverlappedComponent :type "PrimitiveComponent Object Reference") (OtherActor :type "Actor Object Reference") (OtherComp :type "PrimitiveComponent Object Reference") (OtherBodyIndex :type Integer) (bFromSweep :type Boolean) (SweepResult :type "HitResult Structure (by ref)"))
  ;[0 0 0] Remove pin with teeth
  (if (and (`ActorComponent.ComponentHasTag` OtherComp "Teeth") (`/Game/VR_Weapons/Global/Blueprints/Grenade/BP_Grenade.Grabbed` (`self.BP_Grenade`)))
    (`/Engine/EditorBlueprintResources/StandardMacros.DoOnce` false
      (:`Completed`
        (`KismetSystemLibrary.PrintString` "Overlapped" true true (struct :`R` 0.329358 :`G` 1.0 :`B` 0.518123 :`A` 1.0) 8.0)
        (`GameplayStatics.PlaySoundAtLocation` "/Game/VR_Weapons/Flashbang/Audio/Flashbang_pin_remove_teeth_Cue.Flashbang_pin_remove_teeth_Cue" (`SceneComponent.K2_GetComponentLocation` (`self.Overlap`)) (struct) 1.0 1.0 0.0 "/Game/VR_Weapons/Global/Audio/Small_object_Attenuation.Small_object_Attenuation" null null)))))

(event `Server drop`
  ;[0 0 0] Drop
  (`self.Start destroy timer`)
  (`self.Drop pin`))

(event `Drop pin`
  ;[0 0 0] Drop
  ;;[0.494 0.3303 1] 2.2 update: allow pin to drop on all clients
  (if (not (`self.Locally controlled`))
    (`PrimitiveComponent.SetSimulatePhysics` (`self.Pin`) true :!label _label)
    (`self.K2_DetachFromActor` "KeepWorld" "KeepWorld" "KeepWorld")))

(event `/Game/VR_Weapons/Global/Blueprints/BPI_pickup.Drop actor`
  ;[0 0 0] Drop
  (`self.Server drop` :!label _label_2)
  (goto _label))

(event `self.Overlap.OnComponentEndOverlap`
  (params (OverlappedComponent :type "PrimitiveComponent Object Reference") (OtherActor :type "Actor Object Reference") (OtherComp :type "PrimitiveComponent Object Reference") (OtherBodyIndex :type Integer))
  ;[0 0 0] Remove pin with teeth
  (if (and (`/Game/VR_Weapons/Global/Blueprints/Grenade/BP_Grenade.Grabbed` (`self.BP_Grenade`)) (`ActorComponent.ComponentHasTag` OtherComp "Teeth"))
    (`/Game/VR_Weapons/Global/Blueprints/Grenade/BP_Grenade.Lever Pressure Haptics` (`self.BP_Grenade`)) ; lever pressure rumble
    (set `/Game/VR_Weapons/Global/Blueprints/Grenade/BP_Grenade.pin removed` true (`self.BP_Grenade`)) ; tell BP_flashbang the pin has been removed\nand the flashbang is ready to explode when released
    (`GameplayStatics.PlaySoundAtLocation` "/Game/VR_Weapons/Flashbang/Audio/Flashbang_pin_remove_Cue.Flashbang_pin_remove_Cue" (`self.K2_GetActorLocation`) (struct) 1.0 1.0 0.0 "/Game/VR_Weapons/Global/Audio/Small_object_Attenuation.Small_object_Attenuation" null null)
    (goto _label_2)))

(event `Server update pin removed`
  (params (`Attach to` :type "SceneComponent Object Reference") (Hand :type "EControllerHand Enum" :default "Left"))
  ;[0.494 0.3303 1] Update pin removed on server
  (`self.Attach pin` `Attach to` Hand)
  (set `/Game/VR_Weapons/Global/Blueprints/Grenade/BP_Grenade.pin removed` true (`self.BP_Grenade`)))

(event `Start destroy timer`
  ;[0 0 0] Destroy actor
  (`KismetSystemLibrary.K2_SetTimerDelegate` (delegate `Destroy Pin actor when dropped`) 10.0))

(event `Multicast pin removed`
  ;[0.494 0.3303 1] Update pin removed on server
  (`PrimitiveComponent.SetCollisionEnabled` (`self.Overlap`) "NoCollision")
  (if (not (`self.Locally controlled`))
    (`GameplayStatics.PlaySoundAtLocation` "/Game/VR_Weapons/Flashbang/Audio/Flashbang_pin_remove_Cue.Flashbang_pin_remove_Cue" (`self.K2_GetActorLocation`) (struct) 1.0 1.0 0.0 "/Game/VR_Weapons/Global/Audio/Small_object_Attenuation.Small_object_Attenuation" null null)))

(event `Destroy Pin actor when dropped`
  ;[0 0 0] Destroy actor
  (`self.K2_DestroyActor`))

(fn `Attach pin`
  (params (`Attach to` :type "SceneComponent Object Reference") (Hand :type "EControllerHand Enum" :default "Left"))
  (bind _pin (`self.Pin`))
  (`PrimitiveComponent.SetSimulatePhysics` (`self.Pin`) false)
  (`SceneComponent.SetWorldScale3D` _pin (1.0 1.0 1.0))
  (`SceneComponent.K2_AttachToComponent` _pin `Attach to` "PullRingSocket" "SnapToTarget" "SnapToTarget" "KeepWorld" true)
  (`SceneComponent.K2_SetRelativeRotation` (`self.Pullring`) (`KismetMathLibrary.SelectRotator` (struct :`Pitch` 45.0 :`Yaw` 43.0 :`Roll` -55.84) (struct :`Pitch` 45.0 :`Yaw` -43.0 :`Roll` 55.84) (`|EnumEquality` Hand "Right")) false false))

(fn `Pickup actor`
  (params (Hand :type "EControllerHand Enum" :default "Left") (`Grip or grab` :type "/Game/VR_Weapons/Pawn/Blueprints/E_GrabType Enum" :default "NewEnumerator1") (`Motion Controller Actor` :type "/Game/VR_Weapons/Pawn/Blueprints/BP_MotionController Object Reference") (AttachTo :type "SceneComponent Object Reference"))
  (returns (WeaponType :type "/Game/VR_Weapons/Pawn/Blueprints/E_WeaponType Enum") (GunGrabbed :type Boolean))
  (bind _hand (`local.Hand`))
  (bind _attachto (`local.AttachTo`))
  (if (`/Game/VR_Weapons/Global/Blueprints/Grenade/BP_Grenade.Grabbed` (`self.BP_Grenade`))
    (`/Game/VR_Weapons/Pawn/Blueprints/BP_MotionController.RumbleController` `Motion Controller Actor` "/Game/VR_Weapons/Pawn/Haptics/Haptics_single.Haptics_single" 1.0 false) ; pin removal click
    (`/Game/VR_Weapons/Global/Blueprints/Grenade/BP_Grenade.Lever Pressure Haptics` (`self.BP_Grenade`)) ; lever pressure rumble
    (set `/Game/VR_Weapons/Pawn/Blueprints/BP_MotionController.Engage` true `Motion Controller Actor`) ; change the hand animation to engage
    (set `/Game/VR_Weapons/Global/Blueprints/Grenade/BP_Grenade.pin removed` true (`self.BP_Grenade`)) ; tell BP_flashbang the pin has been removed\nand the flashbang is ready to explode when released
    (set `self.Locally controlled` true)
    (`self.Attach pin` _attachto _hand)
    ;[0.494 0.3303 1] Attach on server
    (`self.Server update pin removed` _attachto _hand)
    (`GameplayStatics.PlaySoundAtLocation` "/Game/VR_Weapons/Flashbang/Audio/Flashbang_pin_remove_Cue.Flashbang_pin_remove_Cue" (`self.K2_GetActorLocation`) (struct) 1.0 1.0 0.0 "/Game/VR_Weapons/Global/Audio/Small_object_Attenuation.Small_object_Attenuation" null null)
    (`PrimitiveComponent.SetCollisionEnabled` (`self.Overlap`) "NoCollision")
    (return "NewEnumerator2" false)
    (else
      (return "NewEnumerator0" false))))

(fn `Toggle collision`
  (params (bNewActorEnableCollision :type Boolean))
  (`self.SetActorEnableCollision` bNewActorEnableCollision))

(fn `UserConstructionScript`)