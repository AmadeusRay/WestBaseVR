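; Networked VR pickup cube that motion controllers can grab, carry and throw.
; Pickup attaches the mesh locally with an offset, has the pawn request server ownership, then polls the owner before calling ServerAttach.
; The hand mesh plays a Grab animation while holding and returns to its Animation Blueprint on drop.
; Dropping restores physics and passes velocity to ServerDrop, which replicates the throw and clears the owner.
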(event `Server attach`
  (params (Hand :type "SceneComponent Object Reference"))
  (set `self.hand` Hand)
  (`PrimitiveComponent.SetSimulatePhysics` (`self.StaticMeshComponent`) false)
  (bind _returnvalue (`SceneComponent.K2_AttachToComponent` (`self.StaticMeshComponent`) (`self.hand`) "None" "SnapToTarget" "SnapToTarget" "SnapToTarget" false))
  (if _returnvalue
    (`KismetSystemLibrary.PrintString` "Cube picked up" true true (struct :`R` 0.041247 :`G` 1.0 :`A` 1.0) 8.0)
    (`SceneComponent.K2_SetRelativeTransform` (`self.StaticMeshComponent`) (`self.Offset`) false false)
    (else
      (`KismetSystemLibrary.PrintString` "Cube NOT picked up" true true (struct :`R` 1.0 :`B` 0.012817 :`A` 1.0) 8.0))))

(event `Pickup_Event`
  (params (AttachTo :type "SceneComponent Object Reference") (Hand :type "EControllerHand Enum" :default "Left"))
  (bind _asmotion_controller_pawn (cast `/Game/VR_Weapons/Pawn/Blueprints/MotionControllerPawn` (`GameplayStatics.GetPlayerPawn` 0)))
  (`/Game/VR_Weapons/Pawn/Blueprints/MotionControllerPawn.Server set actor owner in pawn` _asmotion_controller_pawn self)
  (`PrimitiveComponent.SetSimulatePhysics` (`self.StaticMeshComponent`) false)
  (`SceneComponent.K2_AttachToComponent` (`self.StaticMeshComponent`) AttachTo "None" "SnapToTarget" "SnapToTarget" "SnapToTarget" false)
  (`SceneComponent.K2_SetRelativeTransform` (`self.StaticMeshComponent`) (`self.Offset`) false false)
  (if (!= (`self.GetOwner`) null) :!label _label
    (`self.Server attach` AttachTo)
    (else
      (`KismetSystemLibrary.Delay` 0.1)
      (goto _label))))

(event `/Game/VR_Weapons/Global/Blueprints/BPI_pickup.Drop actor`
  (bind _staticmeshcomponent (`self.StaticMeshComponent`))
  (`SkeletalMeshComponent.SetAnimationMode` (`self.Mannequin hand`) "AnimationBlueprint")
  (set `self.Mannequin hand` null)
  (`self.K2_DetachFromActor` "KeepWorld" "KeepWorld" "KeepWorld")
  (`PrimitiveComponent.SetSimulatePhysics` _staticmeshcomponent true)
  (`self.Server drop` (`SceneComponent.GetComponentVelocity` _staticmeshcomponent)))

(event `Server drop`
  (params (Impulse :type "Vector Structure"))
  (`/Game/VR_Weapons/Networking/Networking.Replicate actor throwing` (`self.Networking`) (`self.StaticMeshComponent`) Impulse)
  (`self.SetOwner` null))

(fn `Pickup actor`
  (params (Hand :type "EControllerHand Enum" :default "Left") (`Grip or grab` :type "/Game/VR_Weapons/Pawn/Blueprints/E_GrabType Enum" :default "NewEnumerator1") (`Motion Controller Actor` :type "/Game/VR_Weapons/Pawn/Blueprints/BP_MotionController Object Reference") (AttachTo :type "SceneComponent Object Reference"))
  (returns (WeaponType :type "/Game/VR_Weapons/Pawn/Blueprints/E_WeaponType Enum") (GunGrabbed :type Boolean))
  (bind _handmesh (`/Game/VR_Weapons/Pawn/Blueprints/BP_MotionController.HandMesh` `Motion Controller Actor`))
  (`self.Pickup_Event` AttachTo Hand)
  (set `self.Mannequin hand` _handmesh)
  (`SkeletalMeshComponent.SetAnimationMode` _handmesh "AnimationSingleNode")
  (`SkeletalMeshComponent.SetAnimation` _handmesh "/Game/VR_Weapons/Pawn/Mannequin/Animations/Default/Grab.Grab")
  (return "NewEnumerator0" false))

(fn `UserConstructionScript`)