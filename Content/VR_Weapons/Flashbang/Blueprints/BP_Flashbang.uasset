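; VR flashbang grenade that, on explosion, blinds a player within range and stuns AI.
; A line trace to the player's head gates exposure; likely-indoor blasts also fire bouncing traces to flag close interior proximity.
; Blinding requires that flag or a recently rendered grenade, with duration mapped from explosion distance.
; Quest uses a white-flash widget because mobile lacks post-process support, while other platforms drive a material parameter collection and pawn screen fade.
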(event `self.Grenade explosion`
  (bind _debug_mode (`self.Debug mode`))
  (bind _debug_mode_2 (`self.Debug mode`))
  (bind _flash_intensity (`self.Flash intensity`))
  (bind _debug_mode_3 (`self.Debug mode`))
  (bind _debug_mode_4 (`self.Debug mode`))
  (bind _debug_mode_5 (`self.Debug mode`))
  (bind _debug_mode_6 (`self.Debug mode`))
  (bind _returnvalue (`PrimitiveComponent.WasRecentlyRendered` (`self.Grenade`) 0.1))
  (`|ExecutionSequence`
    (:`then_0`
      (if (`self.Player within range`)
        ;[0 0 0] Check player
        (bind _outhit (`KismetSystemLibrary.LineTraceSingle` :`Start` (`SceneComponent.K2_GetComponentLocation` (`self.Grenade`)) :`End` (`SceneComponent.K2_GetComponentLocation` (`self.Player's head`)) :`TraceChannel` (`self.Trace channel`) :`DrawDebugType` (select `bool` (`self.Debug mode`) :`true` "ForDuration" :!type "EDrawDebugTrace Enum") :`TraceColor` (struct :`R` 1.0 :`G` 0.237876 :`A` 1.0) :`DrawTime` 8.0)) ; line trace to player's head to check if anything is blocking the flashbang
        (bind (_bblockinghit _binitialoverlap _time _distance _location _impactpoint _normal _impactnormal _physmat _hitactor _hitcomponent) (`GameplayStatics.BreakHitResult` _outhit))
        (if (== (`self.Player's head`) _hitcomponent)
          (set `self.Explosion heard` true) ; The player will be deafened temporarily
          (bind _interior (`self.Close proximity check`)) ; inside or outside
          (if _interior
            (for _ (range (`self.Close proximity bounces`))
              (bind _line_trace_hit_player (`self.Bounce line traces inside` (`SceneComponent.K2_GetComponentLocation` (`self.Player's head`)))) ; Bounce line traces off walls/objects in an attempt to reach player
              (if _line_trace_hit_player
                (set `self.Close interior proximity` true)
                (`KismetSystemLibrary.PrintString` "Bounce Reached Player" _debug_mode_2 _debug_mode_2 (struct :`R` 0.006027 :`G` 1.0 :`A` 1.0) 4.0))))
          (if (or (`self.Explosion heard`) (`self.Close interior proximity`))
            ;[0 0 0] Flash visuals
            (`KismetSystemLibrary.Delay` 0.04) ; add slight delay so player can see \nflashbang explode before blindness
            (`KismetSystemLibrary.PrintString` (`KismetStringLibrary.Concat_StrStr` "Flashbang explosion visible = " (`KismetStringLibrary.Conv_BoolToString` _returnvalue)) _debug_mode_5 _debug_mode_5 (struct :`R` 1.0 :`G` 0.381992 :`A` 1.0) 6.0)
            (if (and (or _returnvalue (`self.Close interior proximity`)) (`self.Player within range`))
              (bind _oculus_quest (`/Game/VR_Weapons/Global/Blueprints/GlobalFunctions.IsOculusQuestDevice`))
              (if _oculus_quest
                (bind _asmotion_controller_pawn (cast `/Game/VR_Weapons/Pawn/Blueprints/MotionControllerPawn` (`GameplayStatics.GetPlayerPawn` 0))
                  (:`then`
                    (bind _asflashbang_widget (cast `/Game/VR_Weapons/Flashbang/Blueprints/FlashbangWidget` (`WidgetComponent.GetUserWidgetObject` (`/Game/VR_Weapons/Pawn/Blueprints/MotionControllerPawn.ScreenFlashWidget` _asmotion_controller_pawn)))
                      (:`then`
                        (`/Game/VR_Weapons/Flashbang/Blueprints/FlashbangWidget.WhiteFlash` _asflashbang_widget)
                        (`KismetSystemLibrary.Delay` (`KismetMathLibrary.MapRangeClamped` (`self.Explosion distance`) 0.3 1.0 (`self.Stun duration min`) (`self.Stun duration max`)))
                        (`/Engine/EditorBlueprintResources/StandardMacros.IsValid` _asflashbang_widget
                          (:`Is Valid`
                            (`/Game/VR_Weapons/Flashbang/Blueprints/FlashbangWidget.FadeBack` _asflashbang_widget))))
                      (:`CastFailed`
                        (`KismetSystemLibrary.PrintString` "CAST to widget FAILED" _debug_mode_3 _debug_mode_3 (struct :`R` 1.0 :`G` 0.039531 :`A` 1.0) 3.0))))
                  (:`CastFailed`
                    (`KismetSystemLibrary.PrintString` "CAST to MotionControllerPawn FAILED" _debug_mode_4 _debug_mode_4 (struct :`R` 1.0 :`G` 0.039531 :`A` 1.0) 3.0)))
                (else
                  (`/Game/VR_Weapons/Pawn/Blueprints/MotionControllerPawn.Stop updating flashbang screen fade` (`self.MotionControllerPawn`)) ; Stop screen fade if player has been \nflashbanged again
                  (`KismetMaterialLibrary.SetScalarParameterValue` "/Game/VR_Weapons/Flashbang/Materials/MPC_Flashbang.MPC_Flashbang" "FlashBrightness" _flash_intensity)
                  (`KismetMaterialLibrary.SetScalarParameterValue` "/Game/VR_Weapons/Flashbang/Materials/MPC_Flashbang.MPC_Flashbang" "FlashOverallEffect" _flash_intensity)
                  (`/Game/VR_Weapons/Pawn/Blueprints/MotionControllerPawn.Fade screen back after flashbang` (`self.MotionControllerPawn`) (`KismetMathLibrary.MapRangeClamped` (`self.Explosion distance`) 0.3 1.0 (`self.Stun duration min`) (`self.Stun duration max`)) (`self.Flash intensity`)))))
            (else
              (`KismetSystemLibrary.PrintString` "Flashbang failed to reach local player" _debug_mode_6 _debug_mode_6 (struct :`R` 0.463542 :`G` 0.015916 :`A` 1.0) 6.0)))
          (else
            (`KismetSystemLibrary.PrintString` (`KismetStringLibrary.Concat_StrStr` "Flashbang line trace failed to reach  \nplayer head. Component hit = " (`KismetSystemLibrary.GetPathName` _hitcomponent)) _debug_mode _debug_mode (struct :`R` 1.0 :`G` 0.104032 :`A` 1.0) 5.0)))))
    (:`then_1`
      (`self.Stun AI`))))

(fn `UserConstructionScript`
  (`parent.UserConstructionScript`))