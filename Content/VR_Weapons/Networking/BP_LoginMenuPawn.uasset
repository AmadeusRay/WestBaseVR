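; BP_LoginMenuPawn is the login screen pawn that presents the main menu either in VR or on a flat screen.
; On BeginPlay it uses HMD worn state, Quest detection and StartMenuInVR to choose between a 3D widget with HMD enabled and a viewport widget with mouse cursor.
; It adds left and right weapon input mappings so grab actions click through widget interaction components.
; ToggleServerWidget swaps the 3D main menu and server widgets.
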(event `self.ReceiveBeginPlay`
  (bind _main_menu_widget (`self.Main Menu Widget`))
  (`|ExecutionSequence`
    (:`then_0`
      (`WidgetBlueprintLibrary.SetFocusToGameViewport`)
      (if (`|EnumEquality` (`HeadMountedDisplayFunctionLibrary.GetHMDWornState`) "Worn")
        (set `self.Start menu in VR` true) ; force VR menu if hmd is worn
      )
      (bind _oculus_quest (`/Game/VR_Weapons/Global/Blueprints/GlobalFunctions.IsOculusQuestDevice`))
      (if (or _oculus_quest (`self.Start menu in VR`))
        ;[0.494 0.3303 1] Show/hide 3d menu
        (`WidgetComponent.SetTickMode` _main_menu_widget "Enabled")
        (`HeadMountedDisplayFunctionLibrary.EnableHMD` true)
        (else
          (`WidgetComponent.SetTickMode` _main_menu_widget "Disabled")
          (`HeadMountedDisplayFunctionLibrary.EnableHMD` false)
          ;[0.494 0.3303 1] Create login widget
          (`KismetSystemLibrary.PrintString` "Log in pawn spawned" true true (struct :`R` 0.105407 :`G` 1.0 :`A` 1.0) 6.0)
          (bind _returnvalue (`|CreateWidget` "/Game/VR_Weapons/Networking/Widgets/Login/Widget_MainMenu.Widget_MainMenu_C" (`GameplayStatics.GetPlayerController` 0)))
          (bind _output_get (set `self.Main menu` _returnvalue))
          (`UserWidget.AddToViewport` _output_get 0)
          (set `PlayerController.bShowMouseCursor` true (`GameplayStatics.GetPlayerController` 0)))))
    (:`then_1`
      (bind _aslogin_player_controller (cast `/Game/VR_Weapons/Networking/LoginPlayerController` (`GameplayStatics.GetPlayerController` 0)))
      (bind _returnvalue_2 (pcsubsystem `EnhancedInputLocalPlayerSubsystem` _aslogin_player_controller))
      (`/Engine/EditorBlueprintResources/StandardMacros.IsValid` _returnvalue_2
        (:`Is Valid`
          (`EnhancedInputSubsystemInterface.AddMappingContext` _returnvalue_2 "/Game/VR_Weapons/Pawn/Blueprints/Input/Weapon_left.Weapon_left" 0 (struct))
          (`EnhancedInputSubsystemInterface.AddMappingContext` _returnvalue_2 "/Game/VR_Weapons/Pawn/Blueprints/Input/Weapon_right.Weapon_right" 0 (struct)))))))

(event `EnhancedInput|/Game/VR_Weapons/Pawn/Blueprints/Input/Actions/GrabRight`
  (params (ActionValue :type "Float (double-precision)") (ElapsedSeconds :type "Float (double-precision)") (TriggeredSeconds :type "Float (double-precision)") (InputAction :type "InputAction Object Reference" :default "/Game/VR_Weapons/Pawn/Blueprints/Input/Actions/GrabRight.GrabRight"))
  (bind _rightwidgetinteraction (`self.RightWidgetInteraction`))
  ;[0 0 0] Widget interaction
  (:`Triggered`
    (`WidgetInteractionComponent.PressPointerKey` _rightwidgetinteraction "LeftMouseButton")
    (`KismetSystemLibrary.PrintString` "Right click debug" true true (struct :`G` 1.0 :`B` 0.09978 :`A` 1.0) 1.0))
  (:`Completed`
    (`WidgetInteractionComponent.ReleasePointerKey` _rightwidgetinteraction "LeftMouseButton")))

(event `EnhancedInput|/Game/VR_Weapons/Pawn/Blueprints/Input/Actions/GrabLeft`
  (params (ActionValue :type "Float (double-precision)") (ElapsedSeconds :type "Float (double-precision)") (TriggeredSeconds :type "Float (double-precision)") (InputAction :type "InputAction Object Reference" :default "/Game/VR_Weapons/Pawn/Blueprints/Input/Actions/GrabLeft.GrabLeft"))
  (bind _leftwidgetinteraction (`self.LeftWidgetInteraction`))
  ;[0 0 0] Widget interaction
  (:`Triggered`
    (`WidgetInteractionComponent.PressPointerKey` _leftwidgetinteraction "LeftMouseButton"))
  (:`Completed`
    (`WidgetInteractionComponent.ReleasePointerKey` _leftwidgetinteraction "LeftMouseButton")))

(fn `Toggle server widget`
  (params (bNewVisibility :type Boolean))
  (bind _main_menu_widget (`self.Main Menu Widget`))
  (bind _server_widget (`self.Server Widget`))
  (if bNewVisibility
    (`SceneComponent.SetVisibility` _main_menu_widget false false)
    (`PrimitiveComponent.SetCollisionEnabled` _main_menu_widget "NoCollision")
    (`SceneComponent.SetVisibility` _server_widget true false)
    (else
      (`SceneComponent.SetVisibility` _main_menu_widget true false)
      (`PrimitiveComponent.SetCollisionEnabled` _main_menu_widget "QueryOnly")
      (`SceneComponent.SetVisibility` _server_widget false false)))
  (`WidgetBlueprintLibrary.SetFocusToGameViewport`))

(fn `UserConstructionScript`)