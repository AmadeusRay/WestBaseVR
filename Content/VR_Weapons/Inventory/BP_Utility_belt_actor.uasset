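; VR utility belt inventory with six weapon slots and an ammo slot; server spawns loadout guns with magazines and destroys the belt on death or logout.
; Hand and item overlaps reveal stored items, enlarge slots and trigger haptics; delayed checks hide them again.
; Released items are validated by tag, then attached via AttachOnServer, which updates network ownership.
; Ammo shows only for the held weapon type; Quest can use masked slot materials.
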(event `self.ReceiveBeginPlay`
  (`/Engine/EditorBlueprintResources/ActorMacros.Switch Has Authority`
    (:`Authority`
      ;[0.494 0.3303 1] Run on server
      (`self.Server spawn weapons on begin play`))))

(event `Server spawn weapons on begin play`
  ;[0.494 0.3303 1] Run on server
  (`self.Spawn loadout class weapons`)
  ;[0 0 0] Destroy Utility belt and guns/ammo when player dies or leaves game
  (add `/Game/VR_Weapons/Pawn/Blueprints/MotionControllerPawn.PlayerDead` (`self.MotionControllerPawn`) (delegate `Destroy Utility Belt`))
  (bind _asvrmultiplayer_game_mode (cast `/Game/VR_Weapons/Networking/VRMultiplayerGameMode` (`GameplayStatics.GetGameMode`)))
  (add `/Game/VR_Weapons/Networking/VRMultiplayerGameMode.Player logout` _asvrmultiplayer_game_mode (delegate `Destroy Utility Belt`)))

(event `Destroy Utility Belt`
  ;[0 0 0] Destroy Utility belt and guns/ammo when player dies or leaves game
  (`self.Server destroy all attach items`))

(event `Server destroy all attach items`
  ;[0 0 0] Destroy Utility belt and guns/ammo when player dies or leaves game
  ;;[0.494 0.3303 1] Destroy on server
  (`self.K2_DestroyActor`) ; Destroy Utility belt
)

(event `self.Slot1.OnComponentBeginOverlap`
  (params (OverlappedComponent :type "PrimitiveComponent Object Reference") (OtherActor :type "Actor Object Reference") (OtherComp :type "PrimitiveComponent Object Reference") (OtherBodyIndex :type Integer) (bFromSweep :type Boolean) (SweepResult :type "HitResult Structure (by ref)"))
  ;[0 0 0] Weapons slot overlap begin
  (`self.Overlap begin` OverlappedComponent (`self.Slot Overlapped scale`) OtherActor))

(event `self.Slot2.OnComponentBeginOverlap`
  (params (OverlappedComponent :type "PrimitiveComponent Object Reference") (OtherActor :type "Actor Object Reference") (OtherComp :type "PrimitiveComponent Object Reference") (OtherBodyIndex :type Integer) (bFromSweep :type Boolean) (SweepResult :type "HitResult Structure (by ref)"))
  ;[0 0 0] Weapons slot overlap begin
  (`self.Overlap begin` OverlappedComponent (`self.Slot Overlapped scale`) OtherActor))

(event `self.Ammo slot.OnComponentBeginOverlap`
  (params (OverlappedComponent :type "PrimitiveComponent Object Reference") (OtherActor :type "Actor Object Reference") (OtherComp :type "PrimitiveComponent Object Reference") (OtherBodyIndex :type Integer) (bFromSweep :type Boolean) (SweepResult :type "HitResult Structure (by ref)"))
  (bind _returnvalue (`self.GetAttachParentActor` OtherActor))
  ;[0 0 0] Ammo slot overlap begin
  (if (`self.ActorHasTag` OtherActor "Mag")
    (`SceneComponent.SetRelativeScale3D` OverlappedComponent (0.5 0.5 0.5))
    (`/Engine/EditorBlueprintResources/StandardMacros.IsValid` _returnvalue
      (:`Is Valid`
        (bind _asbp_motion_controller (cast `/Game/VR_Weapons/Pawn/Blueprints/BP_MotionController` _returnvalue)
          (:`then`
            (`/Game/VR_Weapons/Pawn/Blueprints/BP_MotionController.RumbleController` _asbp_motion_controller "/Game/VR_Weapons/Pawn/Haptics/Haptics_single.Haptics_single" 0.3 false))
          (:`CastFailed`
            (bind _asbp_motion_controller_2 (cast `/Game/VR_Weapons/Pawn/Blueprints/BP_MotionController` (`self.GetAttachParentActor` _returnvalue)))
            (`/Game/VR_Weapons/Pawn/Blueprints/BP_MotionController.RumbleController` _asbp_motion_controller_2 "/Game/VR_Weapons/Pawn/Haptics/Haptics_single.Haptics_single" 0.3 false)))))))

(event `self.Slot3.OnComponentBeginOverlap`
  (params (OverlappedComponent :type "PrimitiveComponent Object Reference") (OtherActor :type "Actor Object Reference") (OtherComp :type "PrimitiveComponent Object Reference") (OtherBodyIndex :type Integer) (bFromSweep :type Boolean) (SweepResult :type "HitResult Structure (by ref)"))
  ;[0 0 0] Weapons slot overlap begin
  (`self.Overlap begin` OverlappedComponent (`self.Slot Overlapped scale`) OtherActor))

(event `self.Slot4.OnComponentBeginOverlap`
  (params (OverlappedComponent :type "PrimitiveComponent Object Reference") (OtherActor :type "Actor Object Reference") (OtherComp :type "PrimitiveComponent Object Reference") (OtherBodyIndex :type Integer) (bFromSweep :type Boolean) (SweepResult :type "HitResult Structure (by ref)"))
  ;[0 0 0] Weapons slot overlap begin
  (`self.Overlap begin` OverlappedComponent (`self.Slot Overlapped scale`) OtherActor))

(event `self.Slot5.OnComponentBeginOverlap`
  (params (OverlappedComponent :type "PrimitiveComponent Object Reference") (OtherActor :type "Actor Object Reference") (OtherComp :type "PrimitiveComponent Object Reference") (OtherBodyIndex :type Integer) (bFromSweep :type Boolean) (SweepResult :type "HitResult Structure (by ref)"))
  ;[0 0 0] Weapons slot overlap begin
  (`self.Overlap begin` OverlappedComponent (`self.Slot Overlapped scale`) OtherActor))

(event `self.Ammo slot.OnComponentEndOverlap`
  (params (OverlappedComponent :type "PrimitiveComponent Object Reference") (OtherActor :type "Actor Object Reference") (OtherComp :type "PrimitiveComponent Object Reference") (OtherBodyIndex :type Integer))
  ;[0 0 0] Ammo slot overlap end
  (`SceneComponent.SetRelativeScale3D` OverlappedComponent (0.4 0.4 0.4)))

(event `self.Slot6.OnComponentBeginOverlap`
  (params (OverlappedComponent :type "PrimitiveComponent Object Reference") (OtherActor :type "Actor Object Reference") (OtherComp :type "PrimitiveComponent Object Reference") (OtherBodyIndex :type Integer) (bFromSweep :type Boolean) (SweepResult :type "HitResult Structure (by ref)"))
  ;[0 0 0] Weapons slot overlap begin
  (`self.Overlap begin` OverlappedComponent (`self.Slot Overlapped scale`) OtherActor))

(event `Update Utility belt`
  (params (`Weapon type` :type "/Game/VR_Weapons/Pawn/Blueprints/E_WeaponType Enum" :default "NewEnumerator0"))
  ;[0 0 0] Update visibility of ammo depending on the weapon picked up (called from BP_motioncontroller)
  (set `self.Weapon type in hand` `Weapon type`)
  (for _array_element (`self.GetAttachedActors` true)
    (`self.Update ammo visibility & collision` _array_element)))

(event `self.Slot1.OnComponentEndOverlap`
  (params (OverlappedComponent :type "PrimitiveComponent Object Reference") (OtherActor :type "Actor Object Reference") (OtherComp :type "PrimitiveComponent Object Reference") (OtherBodyIndex :type Integer))
  ;[0 0 0] Weapons slot overlap end
  (`self.Overlap end delayed` OverlappedComponent (`self.Slot Default scale`)))

(event `Hand empty`
  ;[0 0 0] Change weapon type to None when a gun is droppped (called from BP_motioncontroller)
  (set `self.Weapon type in hand` "NewEnumerator0"))

(event `self.Slot2.OnComponentEndOverlap`
  (params (OverlappedComponent :type "PrimitiveComponent Object Reference") (OtherActor :type "Actor Object Reference") (OtherComp :type "PrimitiveComponent Object Reference") (OtherBodyIndex :type Integer))
  ;[0 0 0] Weapons slot overlap end
  (`self.Overlap end delayed` OverlappedComponent (`self.Slot Default scale`)))

(event `Attach on server`
  (params (Item :type "Actor Object Reference") (Slot :type "SceneComponent Object Reference"))
  (bind _returnvalue (`self.GetOwner`))
  ;[0.494 0.3303 1] Attach item to inventory slot on server
  (`self.Attach to slot` Item Slot)
  (message `/Game/VR_Weapons/Global/Blueprints/BPI_pickup.Actor stored in Utility belt` Item true)
  (`KismetSystemLibrary.Delay` 1.0)
  ;[0.494 0.3303 1] Update network owner
  (`self.SetOwner` Item _returnvalue) ; update network owner of actor being attached
  (for _array_element (`self.GetAttachedActors` Item true false)
    (`self.SetOwner` _array_element _returnvalue) ; update network owner of all actors attached \nto the one just added (magazine, silencer, etc)
  ))

(event `self.Slot3.OnComponentEndOverlap`
  (params (OverlappedComponent :type "PrimitiveComponent Object Reference") (OtherActor :type "Actor Object Reference") (OtherComp :type "PrimitiveComponent Object Reference") (OtherBodyIndex :type Integer))
  ;[0 0 0] Weapons slot overlap end
  (`self.Overlap end delayed` OverlappedComponent (`self.Slot Default scale`)))

(event `Item added`
  (params (Slot :type "SceneComponent Object Reference") (NewScale3D :type "Vector Structure"))
  (`self.Overlap end delayed` Slot NewScale3D))

(event `self.Slot4.OnComponentEndOverlap`
  (params (OverlappedComponent :type "PrimitiveComponent Object Reference") (OtherActor :type "Actor Object Reference") (OtherComp :type "PrimitiveComponent Object Reference") (OtherBodyIndex :type Integer))
  ;[0 0 0] Weapons slot overlap end
  (`self.Overlap end delayed` OverlappedComponent (`self.Slot Default scale`)))

(event `self.Slot5.OnComponentEndOverlap`
  (params (OverlappedComponent :type "PrimitiveComponent Object Reference") (OtherActor :type "Actor Object Reference") (OtherComp :type "PrimitiveComponent Object Reference") (OtherBodyIndex :type Integer))
  ;[0 0 0] Weapons slot overlap end
  (`self.Overlap end delayed` OverlappedComponent (`self.Slot Default scale`)))

(event `self.Slot6.OnComponentEndOverlap`
  (params (OverlappedComponent :type "PrimitiveComponent Object Reference") (OtherActor :type "Actor Object Reference") (OtherComp :type "PrimitiveComponent Object Reference") (OtherBodyIndex :type Integer))
  ;[0 0 0] Weapons slot overlap end
  (`self.Overlap end delayed` OverlappedComponent (`self.Slot Default scale`)))

(event `self.Utility belt collision.OnComponentBeginOverlap`
  (params (OverlappedComponent :type "PrimitiveComponent Object Reference") (OtherActor :type "Actor Object Reference") (OtherComp :type "PrimitiveComponent Object Reference") (OtherBodyIndex :type Integer) (bFromSweep :type Boolean) (SweepResult :type "HitResult Structure (by ref)"))
  ;[0 0 0] Toggle utility belt visibility/collision when overlapping with motion controller
  (bind _asbp_motion_controller (cast `/Game/VR_Weapons/Pawn/Blueprints/BP_MotionController` OtherActor))
  (if (== (`self.GetOwner` _asbp_motion_controller) (`self.GetOwner`))
    (`self.Toggle inventory items visibility/collision` false)
    (`self.Update Utility belt` (`self.Weapon type in hand`))
    (set `self.Overlapped` true)))

(event `self.Utility belt collision.OnComponentEndOverlap`
  (params (OverlappedComponent :type "PrimitiveComponent Object Reference") (OtherActor :type "Actor Object Reference") (OtherComp :type "PrimitiveComponent Object Reference") (OtherBodyIndex :type Integer))
  ;[0 0 0] Toggle utility belt visibility/collision when overlapping with motion controller
  (bind _asbp_motion_controller (cast `/Game/VR_Weapons/Pawn/Blueprints/BP_MotionController` OtherActor))
  (if (== (`self.GetOwner`) (`self.GetOwner` _asbp_motion_controller))
    (set `self.Overlapped` false)
    (`KismetSystemLibrary.Delay` 0.4)
    (if (and (not (`self.Overlapped`)) (< (`KismetArrayLibrary.Array_Length` (`PrimitiveComponent.GetOverlappingActors` OverlappedComponent "/Game/VR_Weapons/Pawn/Blueprints/BP_MotionController.BP_MotionController_C")) 1))
      (`self.Toggle inventory items visibility/collision` true))))

(fn `Add item`
  (params (`Item to add` :type "Actor Object Reference") (`Overlapped slot` :type "StaticMeshComponent Object Reference"))
  (bind _debug_mode (`self.Debug mode`))
  (`self.Attach to slot` `Item to add` `Overlapped slot`)
  (`KismetSystemLibrary.PrintString` "Item added" _debug_mode _debug_mode (struct :`R` 0.069388 :`G` 1.0 :`A` 1.0) 4.0)
  (`self.Item added` (`local.Overlapped slot`) (`KismetMathLibrary.SelectVector` (0.4 0.4 0.4) (`self.Slot Default scale`) (== (`local.Overlapped slot`) (`self.Ammo slot`)))))

(fn `Add item to inventory`
  (params (Item :type "Actor Object Reference") (MotionController :type "/Game/VR_Weapons/Pawn/Blueprints/BP_MotionController Object Reference"))
  (returns (Added :type Boolean))
  (locals (`Overlapped slot` :type "StaticMeshComponent Object Reference") (`Parent actor` :type "Actor Object Reference") (`Item added to inventory` :type Boolean))
  ;[0 0 0] Get overlapped slots
  (if (`self.IsOverlappingActor` Item self)
    (for _array_element (`self.Slots`)
      (set `local.Overlapped slot` _array_element)
      ;[0 0 0] Get actor type
      (switch `name` (`|GetArrayItem` (`Actor.Tags` (`local.Item`)))
        (:`Weapon`
          ;[0 0 0] Check slot compatibility
          ;;[1 1 1] Guns
          (bind _add_weapon (`self.Is weapon slot compatible` (`local.Item`) (`local.Overlapped slot`)))
          (if _add_weapon
            (set `local.Item added to inventory` true)
            (message `/Game/VR_Weapons/Global/Blueprints/BPI_pickup.Drop actor` (`local.Item`) :!label _label) ; call drop event to clear motion controller variables in BP_gun
            (`self.Rumble motion controller` (`local.MotionController`))
            (`|ExecutionSequence`
              (:`then_0`
                ;[0.494 0.3303 1] Replicate weapon attach to other players
                (`self.Attach on server` (`local.Item`) (`local.Overlapped slot`)))
              (:`then_1`
                (`self.Add item` (`local.Item`) (`local.Overlapped slot`))
                (return (`local.Item added to inventory`))))))
        (:`Mag`
          ;;[1 1 1] Magazine
          (bind _add_magazine (`self.Is ammo slot compatible` (`local.Overlapped slot`) (`local.Item`)))
          (if _add_magazine
            (set `local.Item added to inventory` true)
            (`self.Update magazine visibility` (`local.Item`))
            (goto _label)))
        (:`Grenade`
          ;;[1 1 1] Grenade
          (bind _add_grenade (`self.Is grenade slot compatible` (`local.Item`) (`local.Overlapped slot`)))
          (if _add_grenade
            (set `local.Item added to inventory` true)
            (goto _label)))))))

(fn `Add magazine to inventory`
  (params (Magazine :type "/Game/VR_Weapons/Global/Blueprints/BP_Magazine Object Reference") (Bullets :type Integer))
  (returns (Added :type Boolean))
  (return false))

(fn `Attach to slot`
  (params (Item :type "Actor Object Reference") (Slot :type "SceneComponent Object Reference"))
  (`self.K2_AttachToComponent` Item Slot "None" "SnapToTarget" "SnapToTarget" "KeepWorld" true)
  (`self.SetActorScale3D` Item (`self.Weapon Attach scale`)))

(fn `Is ammo slot compatible`
  (params (`Overlapped Slot` :type "Object Object Reference") (`Item to add` :type "Actor Object Reference"))
  (returns (`Add Magazine` :type Boolean))
  (bind _ammo_slot (`self.Ammo slot`))
  (return (and (== `Overlapped Slot` _ammo_slot) (`PrimitiveComponent.IsOverlappingActor` _ammo_slot `Item to add`))))

(fn `Is grenade slot compatible`
  (params (Grenade :type "Actor Object Reference") (`Overlapped slot` :type "StaticMeshComponent Object Reference"))
  (returns (`Add grenade` :type Boolean))
  (locals (`Add grenade to inventory` :type Boolean :default false))
  (bind _asbp_grenade (cast `/Game/VR_Weapons/Global/Blueprints/Grenade/BP_Grenade` Grenade))
  (if (and (not (`/Game/VR_Weapons/Global/Blueprints/Grenade/BP_Grenade.pin removed` _asbp_grenade)) (`PrimitiveComponent.IsOverlappingActor` (`local.Overlapped slot`) (`local.Grenade`)))
    (if (== (`SceneComponent.GetChildComponent` `Overlapped slot` 1) null)
      (bind _output_get (set `local.Add grenade to inventory` true :!label _label))
      (return _output_get)
      (elif (`self.ActorHasTag` (`ActorComponent.GetOwner` (`SceneComponent.GetChildComponent` `Overlapped slot` 1)) "Grenade")
        (goto _label)))))

(fn `Is weapon slot compatible`
  (params (`Item to add` :type "Actor Object Reference") (`Overlapped slot` :type "StaticMeshComponent Object Reference"))
  (returns (`Add weapon` :type Boolean))
  (if (and (!= `Overlapped slot` (`self.Ammo slot`)) (!= (`SceneComponent.GetNumChildrenComponents` `Overlapped slot`) 2))
    (if (`PrimitiveComponent.IsOverlappingActor` (`local.Overlapped slot`) (`local.Item to add`))
      (return true)
      (else
        (for _array_element (`self.GetAttachedActors` (`local.Item to add`) true false)
          (if (`PrimitiveComponent.IsOverlappingActor` (`local.Overlapped slot`) _array_element)
            (`|ExecutionSequence`
              (:`then_0`
                (return true))
              (:`then_1`
                (break))))))))
  (return false))

(fn `Overlap begin`
  (params (`Inventory slot` :type "SceneComponent Object Reference") (NewScale3D :type "Vector Structure") (Weapon :type "Actor Object Reference"))
  (`self.Check item` Weapon
    (:`Compatible`
      (`self.Check slot has space` `Inventory slot`
        (:`True`
          ;[0 0 0] Toggle visibility of inventory items and make slot bubble larger to show player the weapon can be added
          (`SceneComponent.SetRelativeScale3D` (`local.Inventory slot`) (`local.NewScale3D`) :!label _label)
          (`self.Toggle inventory items visibility/collision` false)
          (`self.Update Utility belt` (`self.Weapon type in hand`))
          (bind _asbp_gun (cast `/Game/VR_Weapons/Global/Blueprints/BP_Gun` (`local.Weapon`)))
          (bind _primary_motion_controller_bp (`/Game/VR_Weapons/Global/Blueprints/BP_Gun.Primary Motion Controller BP` _asbp_gun))
          (`/Engine/EditorBlueprintResources/StandardMacros.IsValid` _primary_motion_controller_bp ; Check hand ref is still available
            (:`Is Valid`
              (`/Game/VR_Weapons/Pawn/Blueprints/BP_MotionController.RumbleController` _primary_motion_controller_bp "/Game/VR_Weapons/Pawn/Haptics/Haptics_single.Haptics_single" 0.3 false))))
        (:`False`
          (if (and (== (`GameplayStatics.GetObjectClass` (`SceneComponent.GetChildComponent` (`local.Inventory slot`) 1)) "/Game/VR_Weapons/Global/Blueprints/Grenade/BP_Grenade.BP_Grenade_C") (== (`GameplayStatics.GetObjectClass` (`local.Weapon`)) "/Game/VR_Weapons/Global/Blueprints/Grenade/BP_Grenade.BP_Grenade_C"))
            (goto _label)))))))

(fn `Overlap end`
  (params (Target :type "PrimitiveComponent Object Reference") (NewScale3D :type "Vector Structure"))
  (`SceneComponent.SetRelativeScale3D` Target NewScale3D)
  (if (< (`KismetArrayLibrary.Array_Length` (`PrimitiveComponent.GetOverlappingActors` (`self.Utility belt collision`) "/Game/VR_Weapons/Pawn/Blueprints/BP_MotionController.BP_MotionController_C")) 1)
    (`self.Toggle inventory items visibility/collision` true)))

(fn `Rumble motion controller`
  (params (MotionController :type "Actor Object Reference"))
  (bind _asbp_motion_controller (cast `/Game/VR_Weapons/Pawn/Blueprints/BP_MotionController` MotionController))
  (`/Game/VR_Weapons/Pawn/Blueprints/BP_MotionController.RumbleController` _asbp_motion_controller "/Game/VR_Weapons/Pawn/Haptics/Haptics_single.Haptics_single" 0.5 false))

(fn `Spawn loadout class weapons`
  (locals (`Spawned gun` :type "/Game/VR_Weapons/Global/Blueprints/BP_Gun Object Reference"))
  (bind _debug_mode (`self.Debug mode`))
  (bind (_returnvalue_location _returnvalue_rotation) (`KismetMathLibrary.BreakTransform` (`SceneComponent.GetSocketTransform` (`/Game/VR_Weapons/Global/Blueprints/BP_Gun.Gun mesh` (`local.Spawned gun`)) "Magazine" "RTS_World")))
  (if (`self.Spawn weapons`)
    ;[0 0 0] Loop through each available weapon
    (for (_array_element _array_index) (select `int` (`self.Loadout Class`) :`0` (`|MakeArray` "/Game/VR_Weapons/Guns/Handgun/Blueprints/BP_Handgun.BP_Handgun_C" "/Game/VR_Weapons/Guns/Sub-machine_gun/Blueprints/BP_Sub-machine_gun.BP_Sub-machine_gun_C" :!type "Actor Class Reference") :`1` (`|MakeArray` "/Game/VR_Weapons/Guns/Handgun/Blueprints/BP_Handgun.BP_Handgun_C" "/Game/VR_Weapons/Guns/Assault_rifle/Blueprints/BP_Assault_rifle.BP_Assault_rifle_C" :!type "Actor Class Reference") :`2` (`|MakeArray` "/Game/VR_Weapons/Guns/Handgun/Blueprints/BP_Handgun.BP_Handgun_C" "/Game/VR_Weapons/Guns/Sniper_rifle/Blueprints/BP_Sniper_rifle.BP_Sniper_rifle_C" :!type "Actor Class Reference") :`3` (`|MakeArray` "/Game/VR_Weapons/Guns/Shotgun/Blueprints/BP_Shotgun.BP_Shotgun_C" :!type "Actor Class Reference"))
      (`KismetSystemLibrary.PrintString` (`KismetStringLibrary.Concat_StrStr` "Loadout class = " (`KismetStringLibrary.Conv_IntToString` _array_index)) _debug_mode _debug_mode (struct :`G` 0.390625 :`B` 0.302762 :`A` 1.0) 4.0)
      (bind _output (`|GetArrayItem` (`self.Slots`) _array_index))
      (bind (_returnvalue_location_2 _returnvalue_rotation_2) (`KismetMathLibrary.BreakTransform` (`SceneComponent.K2_GetComponentToWorld` _output)))
      ;[0 0 0] Spawn and attach weapon to utility belt
      (bind _returnvalue (`|SpawnActorFromClass` _array_element (`KismetMathLibrary.MakeTransform` _returnvalue_location_2 _returnvalue_rotation_2 (0.2 0.2 0.2)) "AlwaysSpawn" "SelectDefaultAtRuntime" (`self.MotionControllerPawn`) null))
      (bind _asbp_gun (cast `/Game/VR_Weapons/Global/Blueprints/BP_Gun` _returnvalue :!pure true))
      (set `/Game/VR_Weapons/Global/Blueprints/BP_Gun.MotionControllerPawn` (`self.MotionControllerPawn`) _asbp_gun)
      (`/Game/VR_Weapons/Global/Blueprints/BP_Gun.Actor stored in Utility belt` _asbp_gun true)
      (set `local.Spawned gun` _asbp_gun)
      (`/Game/VR_Weapons/Global/Blueprints/BP_Gun.Attach to utility belt` _asbp_gun _output)
      ;[0 0 0] Spawn magazine and attach to gun
      (bind _returnvalue_2 (`|SpawnActorFromClass` (select `/Game/VR_Weapons/Pawn/Blueprints/E_WeaponType` (`/Game/VR_Weapons/Global/Blueprints/BP_Gun.Weapon` _asbp_gun) :`NewEnumerator4` "/Game/VR_Weapons/Guns/Handgun/Blueprints/BP_magazine_Handgun.BP_magazine_Handgun_C" :`NewEnumerator1` "/Game/VR_Weapons/Guns/Sub-machine_gun/Blueprints/BP_Magazine_Sub-machine_gun.BP_Magazine_Sub-machine_gun_C" :`NewEnumerator5` "/Game/VR_Weapons/Guns/Assault_rifle/Blueprints/BP_Magazine_Assault_rifle.BP_Magazine_Assault_rifle_C" :`NewEnumerator3` "/Game/VR_Weapons/Guns/Sniper_rifle/Blueprints/BP_Magazine_Sniper_rifle.BP_Magazine_Sniper_rifle_C" :!type "Actor Class Reference") (`KismetMathLibrary.MakeTransform` _returnvalue_location _returnvalue_rotation) "Undefined" "SelectDefaultAtRuntime" (`self.MotionControllerPawn`) null))
      (bind _asbp_magazine (cast `/Game/VR_Weapons/Global/Blueprints/BP_Magazine` _returnvalue_2 :!pure true))
      (`/Game/VR_Weapons/Global/Blueprints/BP_Magazine.Force insert on spawn` _asbp_magazine (`local.Spawned gun`))
      (set `/Game/VR_Weapons/Global/Blueprints/BP_Magazine.MotionControllerPawn` (`self.MotionControllerPawn`) _asbp_magazine)
      (`/Game/VR_Weapons/Global/Blueprints/BP_Magazine.Actor stored in Utility belt` _asbp_magazine true))))

(fn `Toggle inventory items visibility/collision`
  (params (`Hide actors` :type Boolean))
  (bind _hide_actors (`local.Hide actors`))
  (for _array_element (`self.Slots`)
    (for _array_element_2 (`SceneComponent.GetChildrenComponents` _array_element true)
      (bind _returnvalue (`ActorComponent.GetOwner` _array_element_2))
      (`self.SetActorHiddenInGame` _returnvalue _hide_actors) ; Show weapon actors
      (`self.SetActorEnableCollision` _returnvalue (not _hide_actors)) ; disable collision for all attached actors
      (`self.SetActorEnableCollision` true) ; enable utility belt collision
    )))

(fn `Update ammo visibility & collision`
  (params (`attached actor` :type "Actor Object Reference"))
  (bind _attached_actor (`local.attached actor`))
  (bind _attached_actor_2 (`local.attached actor`))
  (bind _returnvalue (`|EnumEquality` "NewEnumerator6" (`self.Weapon type in hand`)))
  (bind _asbp_magazine (cast `/Game/VR_Weapons/Global/Blueprints/BP_Magazine` `attached actor`)
    (:`then`
      (bind _returnvalue_2 (`|EnumEquality` (`/Game/VR_Weapons/Global/Blueprints/BP_Magazine.MagazineType` _asbp_magazine) (`self.Weapon type in hand`)))
      (`self.SetActorEnableCollision` _attached_actor_2 _returnvalue_2)
      (`self.SetActorHiddenInGame` _attached_actor (not _returnvalue_2)))
    (:`CastFailed`
      (cast `/Game/VR_Weapons/Guns/Shotgun/Blueprints/BP_Shotgun_cartridge` `attached actor`)
      (`self.SetActorEnableCollision` _attached_actor_2 _returnvalue)
      (`self.SetActorHiddenInGame` _attached_actor (not _returnvalue)))))

(fn `Update magazine visibility`
  (params (`Magazine actor` :type "Actor Object Reference"))
  (bind _magazine_actor (`local.Magazine actor`))
  (if (`|EnumInequality` (`self.Weapon type in hand`) "NewEnumerator0")
    (`self.Update ammo visibility & collision` _magazine_actor) ; hide magazine if it doesn't match current weapon in hand\n(only compatible ammo is visible in the utility belt)
    (else
      ;[0 0 0] Check what weapon type is in hand
      (bind _asbp_magazine (cast `/Game/VR_Weapons/Global/Blueprints/BP_Magazine` _magazine_actor)
        (:`then`
          ;;[1 1 1] Set the weapon type for the magazine being added
          (set `self.Weapon type in hand` (`/Game/VR_Weapons/Global/Blueprints/BP_Magazine.MagazineType` _asbp_magazine)))
        (:`CastFailed`
          (cast `/Game/VR_Weapons/Guns/Shotgun/Blueprints/BP_Shotgun_cartridge` _magazine_actor)
          (set `self.Weapon type in hand` "NewEnumerator6")))
      (for _array_element (`self.GetAttachedActors` true)
        (`self.Update ammo visibility & collision` _array_element) ; Only show magazines that match the type added \nand hide all other types
      ))))

(fn `UserConstructionScript`
  (locals (`Use masked material for Oculus Quest optimisation` :type Boolean :default true))
  ;[0 0 0] Set up slots
  (set `self.Slots` (`|MakeArray` (`self.Slot1`) (`self.Slot2`) (`self.Slot3`) (`self.Slot4`) (`self.Slot5`) (`self.Ammo slot`) (`self.Slot6`)))
  ;[0 0 0] Use optimised material for Oculus Quest
  (bind _oculus_quest (`/Game/VR_Weapons/Global/Blueprints/GlobalFunctions.IsOculusQuestDevice`))
  (if (and _oculus_quest (`local.Use masked material for Oculus Quest optimisation`))
    (for _array_element (`self.Slots`)
      (`PrimitiveComponent.SetMaterial` _array_element 0 "/Game/VR_Weapons/Inventory/Materials/MI_UtilityBeltSlot_masked.MI_UtilityBeltSlot_masked") ; Optimise by switching to masked material instead of using transparent if on Quest
    )
    (bind _returnvalue (`PrimitiveComponent.CreateDynamicMaterialInstance` (`self.Ammo slot`) 0 "/Game/VR_Weapons/Inventory/Materials/MI_UtilityBeltSlot_masked.MI_UtilityBeltSlot_masked" "None"))
    (`MaterialInstanceDynamic.SetVectorParameterValue` _returnvalue "Colour2" (struct :`R` 0.184475 :`G` 0.473532 :`B` 1.0 :`A` 1.0))
    (else
      (bind _returnvalue_2 (`PrimitiveComponent.CreateDynamicMaterialInstance` (`self.Ammo slot`) 0 "/Game/VR_Weapons/Inventory/Materials/MI_UtilityBeltSlot.MI_UtilityBeltSlot" "None"))
      (`MaterialInstanceDynamic.SetVectorParameterValue` _returnvalue_2 "Colour2" (struct :`R` 0.184475 :`G` 0.473532 :`B` 1.0 :`A` 1.0)))))