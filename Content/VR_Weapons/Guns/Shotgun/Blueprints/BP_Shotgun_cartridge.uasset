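; VR shotgun shell that a player can grab, drop or throw, and push into a shotgun to load it.
; Pickup snaps it to a hand socket and requests network ownership, retrying with a capped delay loop before attaching on the server.
; Capsule overlap with a shotgun that has magazine space triggers insert feedback, adds a round, frees the hand and destroys the shell.
; Dropping restores physics and replicates throw velocity.
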(event `pickup event`
  ;[0.494 0.3303 1] Set variables and attach on server
  (`self.Wait for network owner to be set`)
  (`self.Server attach` (`self.BP motion controller`) (`self.Hand mesh`)))

(event `Server attach`
  (params (`BP motion controller` :type "/Game/VR_Weapons/Pawn/Blueprints/BP_MotionController Object Reference") (`Hand mesh` :type "SceneComponent Object Reference"))
  ;[0.494 0.3303 1] Set variables and attach on server
  (set `self.BP motion controller` `BP motion controller`)
  (set `self.Hand mesh` `Hand mesh`)
  (`PrimitiveComponent.SetSimulatePhysics` (`self.SM_Cartridge`) false)
  (`SceneComponent.K2_AttachToComponent` (`self.K2_GetRootComponent`) (`self.Hand mesh`) "Shotgun_CartridgeGripSocket" "SnapToTarget" "SnapToTarget" "SnapToTarget" true))

(event `self.Capsule.OnComponentBeginOverlap`
  (params (OverlappedComponent :type "PrimitiveComponent Object Reference") (OtherActor :type "Actor Object Reference") (OtherComp :type "PrimitiveComponent Object Reference") (OtherBodyIndex :type Integer) (bFromSweep :type Boolean) (SweepResult :type "HitResult Structure (by ref)"))
  (bind _debug_mode (`self.Debug mode`))
  (bind _debug_mode_2 (`self.Debug mode`))
  (bind _asbp_shotgun (cast `/Game/VR_Weapons/Guns/Shotgun/Blueprints/BP_Shotgun` OtherActor)
    (:`then`
      (set `self.BP Shotgun` _asbp_shotgun)
      (bind _asbp_magazine_shotgun (cast `/Game/VR_Weapons/Guns/Shotgun/Blueprints/BP_Magazine_shotgun` (`/Game/VR_Weapons/Global/Blueprints/BP_Gun.Magazine` _asbp_shotgun))
        (:`then`
          ;[0 0 0] Check there is space in the gun for a new round
          (if (< (`/Game/VR_Weapons/Global/Blueprints/BP_Magazine.Rounds` _asbp_magazine_shotgun) (`/Game/VR_Weapons/Guns/Shotgun/Blueprints/BP_Magazine_shotgun.Mag max capacity` _asbp_magazine_shotgun))
            (`/Game/VR_Weapons/Guns/Shotgun/Blueprints/BP_Shotgun.Round inserted` _asbp_shotgun) ; play cartirdge elevator anim
            (`|ExecutionSequence`
              (:`then_0`
                ;[0 0 0] vibration
                (bind _bp_motion_controller (`self.BP motion controller`)
                  (:`then`
                    (`/Game/VR_Weapons/Pawn/Blueprints/BP_MotionController.RumbleController` _bp_motion_controller "/Game/VR_Weapons/Pawn/Haptics/Haptics_short.Haptics_short" 0.5 false))
                  (:`else`)))
              (:`then_1`
                (`GameplayStatics.PlaySoundAtLocation` "/Game/VR_Weapons/Guns/Shotgun/Audio/Shotgun_cartridge_insert_Cue.Shotgun_cartridge_insert_Cue" (`self.K2_GetActorLocation`) (struct) 1.0 1.0 0.0 "/Game/VR_Weapons/Global/Audio/Small_object_Attenuation.Small_object_Attenuation" "/Game/VR_Weapons/Global/Audio/WeaponConcurrency.WeaponConcurrency" null)
                (`KismetSystemLibrary.Delay` 0.1)
                (`/Game/VR_Weapons/Guns/Shotgun/Blueprints/BP_Magazine_shotgun.Add round` _asbp_magazine_shotgun) ; Call function to add a new round to the magazine
                (`|ExecutionSequence`
                  (:`then_0`
                    (bind _bp_motion_controller_2 (`self.BP motion controller`)
                      (:`then`
                        ;[0 0 0] update hand to stop gripping
                        (set `/Game/VR_Weapons/Pawn/Blueprints/BP_MotionController.Engage` false _bp_motion_controller_2)
                        (set `/Game/VR_Weapons/Pawn/Blueprints/BP_MotionController.Weapon` "NewEnumerator0" _bp_motion_controller_2)
                        (set `/Game/VR_Weapons/Pawn/Blueprints/BP_MotionController.AttachedActor` null _bp_motion_controller_2))
                      (:`else`)))
                  (:`then_1`
                    (`self.K2_DestroyActor`)))))
            (else
              (`KismetSystemLibrary.PrintString` "No space in magazine" _debug_mode_2 _debug_mode_2 (struct :`R` 0.307292 :`B` 0.003622 :`A` 1.0)))))
        (:`CastFailed`
          (`KismetSystemLibrary.PrintString` "Cast to BP_Magazine_Shotgun failed" _debug_mode _debug_mode (struct :`R` 0.458333 :`B` 0.009311 :`A` 1.0)))))
    (:`CastFailed`
      (`KismetSystemLibrary.PrintString` "Cast to BP_Shotgun failed" _debug_mode _debug_mode (struct :`R` 0.458333 :`B` 0.009311 :`A` 1.0)))))

(event `Server drop`
  (params (Impulse :type "Vector Structure"))
  ;[0.494 0.3303 1] Drop on server
  (`/Game/VR_Weapons/Networking/Networking.Replicate actor throwing` (`self.Networking`) (`self.SM_Cartridge`) Impulse)
  (`self.SetOwner` null))

(event `/Game/VR_Weapons/Global/Blueprints/BPI_pickup.Drop actor`
  (`PrimitiveComponent.SetSimulatePhysics` (`self.SM_Cartridge`) true)
  (`self.K2_DetachFromActor` "KeepWorld" "KeepWorld" "KeepWorld")
  ;[0.494 0.3303 1] Drop on server
  (`self.Server drop` (`SceneComponent.GetComponentVelocity` (`self.SM_Cartridge`))))

(fn `Pickup actor`
  (params (Hand :type "EControllerHand Enum" :default "Left") (`Grip or grab` :type "/Game/VR_Weapons/Pawn/Blueprints/E_GrabType Enum" :default "NewEnumerator1") (`Motion Controller Actor` :type "/Game/VR_Weapons/Pawn/Blueprints/BP_MotionController Object Reference") (AttachTo :type "SceneComponent Object Reference"))
  (returns (WeaponType :type "/Game/VR_Weapons/Pawn/Blueprints/E_WeaponType Enum") (GunGrabbed :type Boolean))
  (bind _debug_mode (`self.Debug mode`))
  (if (and (`|EnumEquality` `Grip or grab` "NewEnumerator1") (== (`self.GetOwner`) null))
    (bind _output_get (set `self.BP motion controller` `Motion Controller Actor`))
    (set `self.Hand mesh` AttachTo)
    (set `/Game/VR_Weapons/Pawn/Blueprints/BP_MotionController.Engage` true _output_get) ; Set hand to engage to update \nblendspace anim
    (`PrimitiveComponent.SetSimulatePhysics` (`self.SM_Cartridge`) false)
    (`SceneComponent.K2_AttachToComponent` (`self.K2_GetRootComponent`) (`self.Hand mesh`) "Shotgun_CartridgeGripSocket" "SnapToTarget" "SnapToTarget" "SnapToTarget" true)
    ;[0.494 0.3303 1] Set network owner
    (bind _asmotion_controller_pawn (cast `/Game/VR_Weapons/Pawn/Blueprints/MotionControllerPawn` (`self.GetOwner` (`self.BP motion controller`)))
      (:`then`
        (`/Game/VR_Weapons/Pawn/Blueprints/MotionControllerPawn.Server set actor owner in pawn` _asmotion_controller_pawn self)
        (`self.pickup event`)
        (return "NewEnumerator6" false))
      (:`CastFailed`
        (`KismetSystemLibrary.PrintString` "CAST TO MOTION CONTROLLER FAILED" _debug_mode _debug_mode (struct :`R` 0.265625 :`G` 0.005475 :`B` 0.01076 :`A` 1.0) 7.0)))))

(fn `UserConstructionScript`)