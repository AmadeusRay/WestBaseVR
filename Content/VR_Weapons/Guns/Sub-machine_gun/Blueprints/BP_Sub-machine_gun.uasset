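; Sub-machine gun weapon Blueprint for VR that specializes a parent gun class.
; The construction script attaches the bolt mesh to the charging handle mesh, keeping its world transform.
; A hand check passes only when the left controller holds the charging handle, controlling whether the hand is shown.
; Handguard grabbing extends the parent's conditions and is blocked while the charging handle is engaged during reloading.
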(event `self.ReceiveBeginPlay`
  (`parent.ReceiveBeginPlay`))

(event `self.ReceiveTick`
  (params (DeltaSeconds :type "Float (single-precision)"))
  (`parent.ReceiveTick` DeltaSeconds))

(fn `Handguard grab conditions`
  (params (Hand :type "/Game/VR_Weapons/Pawn/Blueprints/BP_MotionController Object Reference"))
  (returns (ReturnValue :type Boolean))
  (return (and (`parent.Handguard grab conditions` Hand) (not (`self.Charging Handle engaged`)))))

(fn `Is correct hand`
  (returns (ReturnValue :type Boolean))
  (return (`|EnumEquality` (`/Game/VR_Weapons/Pawn/Blueprints/BP_MotionController.Hand` (`self.Charging handle controller BP`)) "Left")))

(fn `UserConstructionScript`
  (`parent.UserConstructionScript`)
  (`SceneComponent.K2_AttachToComponent` (`self.Bolt mesh`) (`self.Charging handle mesh`) "None" "KeepWorld" "KeepWorld" "KeepWorld" true))