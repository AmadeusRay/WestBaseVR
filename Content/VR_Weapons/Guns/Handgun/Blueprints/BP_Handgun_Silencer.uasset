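; BP_Handgun_Silencer is the handgun-specific silencer Blueprint for the VR weapons set, built on a parent class.
; The construction script runs the parent's logic, then sets the weapon type enum.
; AttachSilencerToGun casts the gun reference to BP_Handgun and snaps the silencer component to the barrel mesh's Silencer socket.
; The event graph holds only disabled placeholder events.
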(fn `Attach silencer to gun`
  (returns (`Successfully attached` :type Boolean))
  (bind _returnvalue (`SceneComponent.K2_AttachToComponent` (`self.Silencer`) (`/Game/VR_Weapons/Guns/Handgun/Blueprints/BP_Handgun.SM_handgun_barrel` (cast `/Game/VR_Weapons/Guns/Handgun/Blueprints/BP_Handgun` (`self.BP_gun`) :!pure true)) "Silencer" "SnapToTarget" "SnapToTarget" "SnapToTarget" true)) ; attach to gun
  (return _returnvalue))

(fn `UserConstructionScript`
  (`parent.UserConstructionScript`)
  (set `self.Weapon Type` "NewEnumerator4"))